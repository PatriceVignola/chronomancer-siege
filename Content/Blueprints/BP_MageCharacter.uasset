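; Mage character Blueprint that adds damage, knockback and healing feedback to the mage.
; On BeginPlay it sets game-only input with a hidden cursor and binds the damageable component's damage event and the hitbox's knockback event.
; Damage plays Wwise audio and a brief blood effect, knockback launches the character along the impact normal, and healing events play dome sound and timed particles.
; The construction script attaches left and right foot Ak audio components to mesh sockets.
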(event Custom|OnDamageTaken_Event_0
  (Class|AkComponent|PostAssociatedAkEvent (Variables|Default|GetDamageAK))
  ;[1 1 1] Blood
  (Components|Activation|Activate (Variables|Default|GetBlood) false)
  (Utilities|FlowControl|Delay 0.2)
  (Components|Activation|Deactivate (Variables|Default|GetBlood)))

(event Custom|OnKnockback_Event_0
  (params (ImpactNormal :type Vector))
  (bind (_x _y _z) (Math|Vector|BreakVector ImpactNormal))
  (Character|LaunchCharacter (Math|Vector|MakeVector (* _x 5e+02) (* _y 5e+02) (+ _z 1e+02)) true true))

(event EventBeginPlay
  (Utilities|FlowControl|Sequence
    (:then_0
      (bind _asplayer_controller (Utilities|Casting|CastToPlayerController (Pawn|GetController)))
      (Input|SetInputModeGameOnly _asplayer_controller)
      (Variables|/Script/Engine.PlayerController|SetbShowMouseCursor _asplayer_controller false))
    (:then_1
      (EventDispatchers|AssignOnDamageTaken (Variables|Default|GetBP_DamageableMage) (delegate Custom|OnDamageTaken_Event_0))
      (EventDispatchers|AssignOnKnockback (Variables|Default|GetDamagableHitbox) (delegate Custom|OnKnockback_Event_0)))))

(event Collision|EventActorBeginOverlap
  (params (OtherActor :type Actor%20Object%20Reference)))

(event EventPlayHealingSound
  (Class|AkGameplayStatics|SpawnAkComponentatLocation "/Game/Audio/Mage_HealingDome.Mage_HealingDome" (Transformation|GetActorLocation) "0, 0, 0" true))

(event EventTick
  (params (DeltaSeconds :type Float%20%28single-precision%29))
  ;[1 1 1] Blood
)

(event EventBPActivateHealingParticles
  (bind _healingparticles (Variables|Default|GetHealingParticles))
  (Components|Activation|Activate _healingparticles false)
  (Utilities|FlowControl|Delay 2.0)
  (Components|Activation|Deactivate _healingparticles))

(fn ConstructionScript
  (Utilities|FlowControl|Sequence
    (:then_0
      (Transformation|AttachComponentToComponent (Variables|Default|GetLeftFootAk) (Variables|Character|GetMesh) "LeftFootSocket" "SnapToTarget" "SnapToTarget" "SnapToTarget" true))
    (:then_1
      (Transformation|AttachComponentToComponent (Variables|Default|GetRightFootAk) (Variables|Character|GetMesh) "RightFootSocket" "SnapToTarget" "SnapToTarget" "SnapToTarget" true))))
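; BP_ActivablePillar is a pillar actor that visually and audibly reflects three states: desactivated, activated and active.
; Each state event swaps material slot 1 on both the pillar mesh and the logo mesh.
; Activation also posts the DistortionAK component's Wwise event and runs a half-second burst of Sparks.
; The Blueprint only handles presentation, with no logic here deciding when the state changes.
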(event EventBeginPlay)

(event Collision|EventActorBeginOverlap
  (params (OtherActor :type Actor%20Object%20Reference)))

(event EventPillarActivated
  (Class|AkComponent|PostAssociatedAkEvent (Variables|Default|GetDistortionAK))
  (Rendering|Material|SetMaterial (Variables|Default|GetStaticMesh) 1 "/Game/Materials/Final_Materials/Pillard-Activated.Pillard-Activated")
  (Rendering|Material|SetMaterial (Variables|Default|GetSM_Logo-Mesh) 1 "/Game/Materials/Final_Materials/Pillard-Activated.Pillard-Activated")
  (Components|Activation|Activate (Variables|Default|GetSparks) false)
  (Utilities|FlowControl|Delay 0.5)
  (Components|Activation|Deactivate (Variables|Default|GetSparks)))

(event EventPillarDesactivated
  (Rendering|Material|SetMaterial (Variables|Default|GetStaticMesh) 1 "/Game/Materials/Final_Materials/Pillard-Desactivated.Pillard-Desactivated")
  (Rendering|Material|SetMaterial (Variables|Default|GetSM_Logo-Mesh) 1 "/Game/Materials/Final_Materials/Pillard-Desactivated.Pillard-Desactivated"))

(event EventPillarActive
  (Rendering|Material|SetMaterial (Variables|Default|GetStaticMesh) 1 "/Game/Materials/Final_Materials/Pillard-Active.Pillard-Active")
  (Rendering|Material|SetMaterial (Variables|Default|GetSM_Logo-Mesh) 1 "/Game/Materials/Final_Materials/Pillard-Active.Pillard-Active"))

(fn ConstructionScript)
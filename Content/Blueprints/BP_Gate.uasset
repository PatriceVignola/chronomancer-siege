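; BP_Gate is an activable gate that opens and closes on request and reflects the state of its linked pillar.
; On BeginPlay it caches its mesh's AnimBP_Gate and binds to open, close and pillar events.
; Open and close requests toggle the animation's door state and play Wwise unlock or lock sounds, with closing reported finished after a fixed delay.
; Pillar events swap a mesh material slot between active, activated and deactivated looks.
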(event Custom|OnOpenActivableRequested_Event_0
  (Variables|/Game/Models/AnimatedObjects/AnimBP_Gate.AnimBP_Gate_C|SetDoor1State (Variables|Default|GetGateAnim) true)
  (Class|AkComponent|PostAssociatedAkEvent (Variables|Default|GetUnlockAK)))

(event Custom|PillardActive
  (Rendering|Material|SetMaterial (Variables|Character|GetMesh) 1 "/Game/Materials/Final_Materials/Pillard-Active.Pillard-Active"))

(event Custom|PillardActivated
  (Rendering|Material|SetMaterial (Variables|Character|GetMesh) 1 "/Game/Materials/Final_Materials/Pillard-Activated.Pillard-Activated"))

(event Custom|PillardDeactivated
  (Rendering|Material|SetMaterial (Variables|Character|GetMesh) 1 "/Game/Materials/Final_Materials/Pillard-Desactivated.Pillard-Desactivated"))

(event Custom|OnCloseActivableRequested_Event_0
  (Variables|/Game/Models/AnimatedObjects/AnimBP_Gate.AnimBP_Gate_C|SetDoor1State (Variables|Default|GetGateAnim) false)
  (Development|PrintString "ACTIVATEEEEEEEEEEEEEE")
  (Class|AkComponent|PostAssociatedAkEvent (Variables|Default|GetLockAK))
  (Utilities|FlowControl|Delay 6.0)
  (Class|Gate|NotifyDoorFinishedClosing))

(event EventBeginPlay
  (bind _asanim_bp_gate (Utilities|Casting|CastToAnimBP_Gate (Components|SkeletalMesh|GetAnimInstance (Variables|Character|GetMesh))))
  (Variables|Default|SetGateAnim _asanim_bp_gate)
  (EventDispatchers|BindEventtoOnOpenActivableRequested (delegate Custom|OnOpenActivableRequested_Event_0))
  (EventDispatchers|BindEventtoOnCloseActivableRequested (delegate Custom|OnCloseActivableRequested_Event_0))
  (EventDispatchers|BindEventtoOnPillarActivated (delegate Custom|PillardActivated))
  (EventDispatchers|BindEventtoOnPillarActive (delegate Custom|PillardActive))
  (EventDispatchers|BindEventtoOnPillarDeactivated (delegate Custom|PillardDeactivated)))

(event Collision|EventActorBeginOverlap
  (params (OtherActor :type Actor%20Object%20Reference)))

(event EventTick
  (params (DeltaSeconds :type Float%20%28single-precision%29)))

(fn ConstructionScript)
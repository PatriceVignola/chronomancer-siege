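; BP_WarriorCharacter is the warrior character Blueprint, handling combat feedback and record/rewind screen effects.
; On BeginPlay it sets game-only input and binds damageable, hitbox, Recordable and Rewindable events, driving hit/death animation, knockback launches, damage feedback and post-process toggles.
; Record post-process toggles go through RPC events, while rewind toggles apply directly.
; Separate events play indexed Wwise attack sounds and timed healing particles; construction socket-attaches sword and foot audio.
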(event Custom|OnEnableRecordPostProcessRequested_Event_0
  (CallFunction|RPCEnableRecordPostProcess))

(event Custom|OnDamageTaken_Event_0
  (Class|AkComponent|PostAssociatedAkEvent (Variables|Default|GetDamageAK))
  (Components|Activation|Activate (Variables|Default|GetBloodParticles) true)
  (Utilities|FlowControl|Delay 0.2)
  (Components|Activation|Deactivate (Variables|Default|GetBloodParticles)))

(event Custom|RPC_EnableRecordPostProcess
  (Variables|/Script/Engine.PostProcessComponent|SetbEnabled (Variables|/Script/Academia2017.CustomPostProcessComponent|GetPostProcess (Variables|Default|GetBP_RecordPostProcess)) true))

(event Custom|OnDisableRewindPostProcessRequested_Event_0
  (Variables|/Script/Engine.PostProcessComponent|SetbEnabled (Variables|Default|GetPostProcess_Rewinding) false))

(event Custom|RPC_DisableRecordPostProcess
  (Variables|/Script/Engine.PostProcessComponent|SetbEnabled (Variables|/Script/Academia2017.CustomPostProcessComponent|GetPostProcess (Variables|Default|GetBP_RecordPostProcess)) false))

(event Custom|OnDisableRecordPostProcessRequested_Event_0
  (CallFunction|RPCDisableRecordPostProcess))

(event Custom|OnEnableRewindPostProcessRequested_Event_0
  (Variables|/Script/Engine.PostProcessComponent|SetbEnabled (Variables|Default|GetPostProcess_Rewinding) true))

(event Custom|HealthChange
  (params (health :type Float%20%28single-precision%29))
  (Default|CallOnAnimHealthChange (<= health 0.0) (Variables|/Script/Academia2017.DamagableHitbox|GetHitLocation (Variables|Default|GetDamagableHitbox)) (Variables|/Script/Academia2017.DamagableHitbox|GetHasBeenHit (Variables|Default|GetDamagableHitbox))))

(event Custom|CustomEvent_0
  (params (ImpactNormal :type Vector))
  (bind (_x _y _z) (Math|Vector|BreakVector ImpactNormal))
  (Character|LaunchCharacter (Math|Vector|MakeVector (* _x 5e+02) (* _y 5e+02) (+ _z 1e+02)) true true))

(event EventBeginPlay
  (bind _recordable (Variables|Default|GetRecordable))
  (bind _rewindable (Variables|Default|GetRewindable))
  (Utilities|FlowControl|Sequence
    (:then_0
      (bind _asplayer_controller (Utilities|Casting|CastToPlayerController (Pawn|GetController)))
      (Input|SetInputModeGameOnly _asplayer_controller)
      (Variables|/Script/Engine.PlayerController|SetbShowMouseCursor _asplayer_controller false))
    (:then_1
      (EventDispatchers|BindEventtoOnHealthChanged (Variables|Default|GetBP_DamageableWarrior) (delegate Custom|HealthChange)))
    (:then_2
      (EventDispatchers|AssignOnEnableRecordPostProcessRequested _recordable (delegate Custom|OnEnableRecordPostProcessRequested_Event_0)))
    (:then_3
      (EventDispatchers|AssignOnDisableRecordPostProcessRequested _recordable (delegate Custom|OnDisableRecordPostProcessRequested_Event_0)))
    (:then_4
      (EventDispatchers|AssignOnEnableRewindPostProcessRequested _rewindable (delegate Custom|OnEnableRewindPostProcessRequested_Event_0)))
    (:then_5
      (EventDispatchers|AssignOnDisableRewindPostProcessRequested _rewindable (delegate Custom|OnDisableRewindPostProcessRequested_Event_0)))
    (:then_6
      (EventDispatchers|AssignOnDamageTaken (Variables|Default|GetBP_DamageableWarrior) (delegate Custom|OnDamageTaken_Event_0)))
    (:then_7
      (EventDispatchers|BindEventtoOnKnockback (Variables|Default|GetDamagableHitbox) (delegate Custom|CustomEvent_0)))))

(event EventBPActivateHealingParticles
  (bind _healingparticles (Variables|Default|GetHealingParticles))
  (Components|Activation|Activate _healingparticles false)
  (Utilities|FlowControl|Delay 2.0)
  (Components|Activation|Deactivate _healingparticles))

(event EventTick
  (params (DeltaSeconds :type Float%20%28single-precision%29)))

(event EventPlayLightAttackSound
  (params (attackIndex :type Integer))
  (Class|AkComponent|PostAkEvent (Variables|Default|GetSwordAk) (Utilities|Array|Get(acopy) (Variables|Default|GetLightAttackAudioEvents) attackIndex)))

(event EventPlayHeavyAttackSound
  (params (attackIndex :type Integer))
  (Class|AkComponent|PostAkEvent (Variables|Default|GetSwordAk) (Utilities|Array|Get(acopy) (Variables|Default|GetHeavyAttackAudioEvents) attackIndex)))

(fn ConstructionScript
  (Utilities|FlowControl|Sequence
    (:then_0
      (Transformation|AttachComponentToComponent (Variables|Default|GetSwordComponent) (Variables|Character|GetMesh) "SwordSocket" "SnapToTarget" "SnapToTarget" "SnapToTarget" true))
    (:then_1
      (Transformation|AttachComponentToComponent (Variables|Default|GetLeftFootAk) (Variables|Character|GetMesh) "LeftFootSocket" "SnapToTarget" "SnapToTarget" "SnapToTarget" true))
    (:then_2
      (Transformation|AttachComponentToComponent (Variables|Default|GetRightFootAk) (Variables|Character|GetMesh) "RightFootSocket" "SnapToTarget" "SnapToTarget" "SnapToTarget" true))))
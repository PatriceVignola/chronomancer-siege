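; Secarian Worker enemy Blueprint that reacts to its damageable component's health, damage, death and revive events.
; Death hides the health widget, makes the capsule ignore pawns, unregisters the AI bucket and plays a Wwise sound, while revive restores widget and collision.
; Construction snaps the attack hitbox and foot audio to mesh sockets, with functions toggling hitbox damage.
; Warrior and Mage are cached at BeginPlay, but the widget-facing logic using them is disconnected.
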(event Custom|OnHealthChangedEvent
  (params (health :type Float%20%28single-precision%29))
  (Default|CallOnAnimHealthChanged (<= health 0.0)))

(event Custom|OnDied_Event_0
  (Development|SetHiddeninGame (Variables|Default|GetHealthWidget) true false)
  (Collision|SetCollisionResponsetoChannel (Variables|Default|GetCapsuleComponent) "ECC_Pawn" "ECR_Ignore")
  (Class|AIBucketComponent|UnregisterBucket (Variables|Default|GetAIBucket))
  (Class|AkComponent|PostAssociatedAkEvent (Variables|Default|GetDeathSound)))

(event Custom|OnDamageTaken_Event_0
  (Class|AkComponent|PostAssociatedAkEvent (Variables|Default|GetDamageAK)))

(event Custom|OnRevived_Event_0
  (Development|SetHiddeninGame (Variables|Default|GetHealthWidget) false false)
  (Collision|SetCollisionResponsetoChannel (Variables|Default|GetCapsuleComponent) "ECC_Pawn" "ECR_Block"))

(event EventBeginPlay
  (bind _bp_workerdamageable (Variables|Default|GetBP_WorkerDamageable))
  (Utilities|FlowControl|Sequence
    (:then_0
      (EventDispatchers|AssignOnRevived _bp_workerdamageable (delegate Custom|OnRevived_Event_0))
      (EventDispatchers|AssignOnDied _bp_workerdamageable (delegate Custom|OnDied_Event_0))
      (EventDispatchers|BindEventtoOnHealthChanged _bp_workerdamageable (delegate Custom|OnHealthChangedEvent))
      (Utilities|FlowControl|Sequence
        (:then_0
          (bind _outactors (Actor|GetAllActorsOfClass "/Game/Blueprints/BP_WarriorCharacter.BP_WarriorCharacter_C"))
          (Variables|Default|SetWarrior (Utilities|Array|Get(acopy) _outactors)))
        (:then_1
          (bind _outactors_2 (Actor|GetAllActorsOfClass "/Game/Blueprints/BP_MageCharacter.BP_MageCharacter_C"))
          (Variables|Default|SetMage (Utilities|Array|Get(acopy) _outactors_2)))))
    (:then_1
      (EventDispatchers|AssignOnDamageTaken (Variables|Default|GetBP_WorkerDamageable) (delegate Custom|OnDamageTaken_Event_0)))))

(event Collision|EventActorBeginOverlap
  (params (OtherActor :type Actor%20Object%20Reference)))

(event EventTick
  (params (DeltaSeconds :type Float%20%28single-precision%29)))

(fn ConstructionScript
  (Utilities|FlowControl|Sequence
    (:then_0
      (Transformation|AttachComponentToComponent (Variables|Default|GetAttackHitBox) (Variables|Character|GetMesh) "LeftArm1" "SnapToTarget" "SnapToTarget" "SnapToTarget" true))
    (:then_1
      (Transformation|AttachComponentToComponent (Variables|Default|GetLeftFootAK) (Variables|Character|GetMesh) "LeftFootSocket" "SnapToTarget" "SnapToTarget" "SnapToTarget" true))
    (:then_2
      (Transformation|AttachComponentToComponent (Variables|Default|GetRightFootAK) (Variables|Character|GetMesh) "RightFootSocket" "SnapToTarget" "SnapToTarget" "SnapToTarget" true))))

(fn EnableDamage
  (Variables|/Script/Academia2017.AttackHitbox|SetCanDamage (Variables|Default|GetAttackHitBox) true))

(fn DisableDamage
  (Variables|/Script/Academia2017.AttackHitbox|SetCanDamage (Variables|Default|GetAttackHitBox) false))

(fn SetAttackDamage
  (Variables|/Script/Academia2017.AttackHitbox|SetBaseDamage (Variables|Default|GetAttackHitBox) (Variables|Default|GetDamageAmount)))

(fn SetRotation)
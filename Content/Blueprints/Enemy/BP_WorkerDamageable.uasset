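; BP_WorkerDamageable is a health component for the Secarian Worker enemy that drives the health bar on its owner.
; On BeginPlay it caches the EnemyHealth widget from the worker's HealthWidget.
; With authority only, it then binds to OnHealthChanged and sets health to MaxHealth.
; Each health change event updates the widget's percent from health over MaxHealth, with no Tick logic.
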(event Custom|OnHealthChangedEvent
  (params (health :type Float%20%28single-precision%29))
  (Default|SetPercent (Variables|Default|GetWidget) (/ health (Variables|Default|GetMaxHealth))))

(event EventBeginPlay
  (bind _asbp_secarian_worker (Utilities|Casting|CastToBP_Secarian_Worker (Components|GetOwner)))
  (bind _asenemy_health (Utilities|Casting|CastToEnemyHealth (UserInterface|GetUserWidgetObject (Variables|/Game/Blueprints/Enemy/BP_Secarian_Worker.BP_Secarian_Worker_C|GetHealthWidget _asbp_secarian_worker))))
  (Variables|Default|SetWidget _asenemy_health)
  (if (Ability|HasAuthority (Components|GetOwner))
    (EventDispatchers|AssignOnHealthChanged (delegate Custom|OnHealthChangedEvent))
    (Class|DamageableCharacterComponent|SetHealth (Variables|Default|GetMaxHealth))))

(event EventTick
  (params (DeltaSeconds :type Float%20%28single-precision%29)))
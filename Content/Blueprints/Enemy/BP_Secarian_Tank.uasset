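; Secarian Tank enemy Blueprint that handles damage feedback, death and revival collision, and attack hitboxes.
; The construction script snaps two hitboxes and Wwise audio components for attacks and four feet onto mesh sockets.
; BPTankDamageable events drive a hit sound with a brief particle burst, and toggle capsule Pawn and custom-channel responses between ignore on death and block on revival.
; SetCanDamage switches both hitboxes together.
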(event Custom|OnDied_Event_0
  (bind _capsulecomponent (Variables|Default|GetCapsuleComponent))
  (Collision|SetCollisionResponsetoChannel _capsulecomponent "ECC_Pawn" "ECR_Ignore")
  (Collision|SetCollisionResponsetoChannel _capsulecomponent "ECC_GameTraceChannel10" "ECR_Ignore"))

(event Custom|OnRevived_Event_0
  (bind _capsulecomponent (Variables|Default|GetCapsuleComponent))
  (Collision|SetCollisionResponsetoChannel _capsulecomponent "ECC_Pawn" "ECR_Block")
  (Collision|SetCollisionResponsetoChannel _capsulecomponent "ECC_GameTraceChannel10" "ECR_Block"))

(event Custom|OnDamageTaken_Event_0
  (Class|AkComponent|PostAssociatedAkEvent (Variables|Default|GetDamageAK))
  (Components|Activation|Activate (Variables|Default|GetParticleSystem) true)
  (Utilities|FlowControl|Delay 0.5)
  (Components|Activation|Deactivate (Variables|Default|GetParticleSystem)))

(event EventBeginPlay
  (Utilities|FlowControl|Sequence
    (:then_0
      (EventDispatchers|AssignOnDied (Variables|Default|GetBP_TankDamageable) (delegate Custom|OnDied_Event_0))
      (EventDispatchers|AssignOnRevived (Variables|Default|GetBP_TankDamageable) (delegate Custom|OnRevived_Event_0)))
    (:then_1
      (EventDispatchers|AssignOnDamageTaken (Variables|Default|GetBP_TankDamageable) (delegate Custom|OnDamageTaken_Event_0)))))

(event Collision|EventActorBeginOverlap
  (params (OtherActor :type Actor%20Object%20Reference)))

(event EventTick
  (params (DeltaSeconds :type Float%20%28single-precision%29)))

(fn ConstructionScript
  (bind _mesh (Variables|Character|GetMesh))
  (Utilities|FlowControl|Sequence
    (:then_0
      (Transformation|AttachComponentToComponent (Variables|Default|GetAttackHitbox) (Variables|Character|GetMesh) "AttackSocket1" "SnapToTarget" "SnapToTarget" "SnapToTarget" true)
      (Transformation|AttachComponentToComponent (Variables|Default|GetAttackHitbox2) (Variables|Character|GetMesh) "AttackSocket2" "SnapToTarget" "SnapToTarget" "SnapToTarget" true)
      (Transformation|AttachComponentToComponent (Variables|Default|GetLeftAttackAK) (Variables|Character|GetMesh) "AttackSocket1" "SnapToTarget" "SnapToTarget" "SnapToTarget" true)
      (Transformation|AttachComponentToComponent (Variables|Default|GetRightAttackAK) (Variables|Character|GetMesh) "AttackSocket2" "SnapToTarget" "SnapToTarget" "SnapToTarget" true))
    (:then_1
      (Transformation|AttachComponentToComponent (Variables|Default|GetRearLeftFootAK) _mesh "RearLeftFootSocket" "SnapToTarget" "SnapToTarget" "SnapToTarget" true))
    (:then_2
      (Transformation|AttachComponentToComponent (Variables|Default|GetRearRightFootAK) _mesh "RearRightFootSocket" "SnapToTarget" "SnapToTarget" "SnapToTarget" true))
    (:then_3
      (Transformation|AttachComponentToComponent (Variables|Default|GetFrontLeftFootAK) _mesh "FrontLeftFootSocket" "SnapToTarget" "SnapToTarget" "SnapToTarget" true))
    (:then_4
      (Transformation|AttachComponentToComponent (Variables|Default|GetFrontRightFootAK) _mesh "FrontRightFootSocket" "SnapToTarget" "SnapToTarget" "SnapToTarget" true))))

(fn SetCanDamage
  (params (CanDamage :type Boolean))
  (Utilities|FlowControl|Sequence
    (:then_0
      (Class|AttackHitbox|SetCanDamage (Variables|Default|GetAttackHitbox2) CanDamage))
    (:then_1
      (Class|AttackHitbox|SetCanDamage (Variables|Default|GetAttackHitBox) CanDamage))))
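; Damageable component for the Sequarian Lord enemy that ties its health value to the Lord's health bar widget.
; On BeginPlay it casts its owner to the Lord and caches the EnemyHealth widget from the Health widget component.
; Only with authority does it bind the health-changed event and set health to maximum.
; That event sets the widget's percent from current over maximum health.
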(event Custom|OnHealthChangedEvent
  (params (health :type Float%20%28single-precision%29))
  (Default|SetPercent (Variables|Default|GetWidget) (/ health (Variables|Default|GetMaxHealth))))

(event EventBeginPlay
  (bind _asbp_sequarian_lord (Utilities|Casting|CastToBP_Sequarian_Lord (Components|GetOwner)))
  (bind _asenemy_health (Utilities|Casting|CastToEnemyHealth (UserInterface|GetUserWidgetObject (Variables|/Game/Blueprints/Enemy/BP_Sequarian_Lord.BP_Sequarian_Lord_C|GetHealth _asbp_sequarian_lord))))
  (Variables|Default|SetWidget _asenemy_health)
  (if (Ability|HasAuthority (Components|GetOwner))
    (EventDispatchers|AssignOnHealthChanged (delegate Custom|OnHealthChangedEvent))
    (Class|DamageableCharacterComponent|SetHealth (Variables|Default|GetMaxHealth))))

(event EventTick
  (params (DeltaSeconds :type Float%20%28single-precision%29)))
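; Enemy Blueprint for the Secarian Assassin, handling health reactions, death and revive state, and combat audio.
; Damageable component events drive animation health notifications, toggle the health widget and capsule Pawn collision, and unregister the AI bucket on death.
; Hit box impact and damage-taken events post Wwise sounds.
; The construction script snaps the attack hit box to the left arm and footstep audio components to foot sockets.
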(event Custom|OnHealthChangedEvent
  (params (health :type Float%20%28single-precision%29))
  (Default|CallOnAnimHealthChanged (<= health 0.0)))

(event Custom|OnDamageTaken_Event_0
  (Class|AkComponent|PostAssociatedAkEvent (Variables|Default|GetDamageAK)))

(event Custom|CustomEvent_1
  (Development|SetHiddeninGame (Variables|Default|GetHealthWidget) true false)
  (Collision|SetCollisionResponsetoChannel (Variables|Default|GetCapsuleComponent) "ECC_Pawn" "ECR_Ignore")
  (Class|AIBucketComponent|UnregisterBucket (Variables|Default|GetAIBucket)))

(event Custom|CustomEvent
  (Development|SetHiddeninGame (Variables|Default|GetHealthWidget) false false)
  (Collision|SetCollisionResponsetoChannel (Variables|Default|GetCapsuleComponent) "ECC_Pawn" "ECR_Block"))

(event Custom|OnPlayImpactSoundRequested_Event_0
  (Class|AkComponent|PostAssociatedAkEvent (Variables|Default|GetAttackAK)))

(event EventBeginPlay
  (bind _bp_workerdamageable (Variables|Default|GetBP_WorkerDamageable))
  (Utilities|FlowControl|Sequence
    (:then_0
      (EventDispatchers|AssignOnRevived _bp_workerdamageable (delegate Custom|CustomEvent))
      (EventDispatchers|AssignOnDied _bp_workerdamageable (delegate Custom|CustomEvent_1))
      (EventDispatchers|BindEventtoOnHealthChanged (Variables|Default|GetBP_WorkerDamageable) (delegate Custom|OnHealthChangedEvent)))
    (:then_1
      (EventDispatchers|AssignOnPlayImpactSoundRequested (Variables|Default|GetAttackHitBox) (delegate Custom|OnPlayImpactSoundRequested_Event_0)))
    (:then_2
      (EventDispatchers|AssignOnDamageTaken (Variables|Default|GetBP_WorkerDamageable) (delegate Custom|OnDamageTaken_Event_0)))))

(event Collision|EventActorBeginOverlap
  (params (OtherActor :type Actor%20Object%20Reference)))

(fn ConstructionScript
  (Utilities|FlowControl|Sequence
    (:then_0
      (Transformation|AttachComponentToComponent (Variables|Default|GetAttackHitBox) (Variables|Character|GetMesh) "LeftArm1" "SnapToTarget" "SnapToTarget" "SnapToTarget" true))
    (:then_1
      (Transformation|AttachComponentToComponent (Variables|Default|GetLeftFootAK) (Variables|Character|GetMesh) "LeftFootSocket" "SnapToTarget" "SnapToTarget" "SnapToTarget" true))
    (:then_2
      (Transformation|AttachComponentToComponent (Variables|Default|GetRightFootAK) (Variables|Character|GetMesh) "RightFootSocket" "SnapToTarget" "SnapToTarget" "SnapToTarget" true))))
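; Sequarian Lord boss enemy that starts hidden and non-blocking to pawns until activated, with toggleable attack hitboxes.
; Construction attaches hitboxes, egg-spawn and weak-point containers, and audio components to mesh sockets.
; Activation and flight-stop route through authority checks to RPCs; activation reveals the boss, removes its defense hitbox and enables collision.
; BPBossDamageable events drive the weak-point material's health percentage, blood, hurt and death sounds, and drop pawn collision on death.
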(event Custom|RPC_OnBossActive
  (Variables|Default|SetIsActive true)
  (Utilities|FlowControl|DoOnce false
    (:Completed
      (Rendering|SetActorHiddenInGame false)
      (Components|DestroyComponent (Variables|Default|GetDefenseHitBox))
      (Collision|SetCollisionResponsetoChannel (Variables|Character|GetMesh) "ECC_Pawn" "ECR_Block"))))

(event Custom|RPC_StopFlying
  (Class|AkComponent|PostAssociatedAkEvent (Variables|Default|GetFlightAKEnd))
  (Class|AkComponent|Stop (Variables|Default|GetFlightAK)))

(event Custom|CustomEvent_0
  (params (health :type Float%20%28single-precision%29))
  (Rendering|Material|SetScalarParameterValue (Variables|Default|GetWeakPointMaterial) "HealthPercentage" (/ health (Variables|/Script/Academia2017.DamageableCharacterComponent|GetMaxHealth (Variables|Default|GetBP_BossDamageable))) :!class /Script/Engine.MaterialInstanceDynamic))

(event Custom|Activate_Event
  (Networking|SwitchHasAuthority
    (:Authority
      (CallFunction|RPConBossActive))
    (:Remote
      (CallFunction|ServeronBossActive))))

(event Custom|OnDied_Event_0
  (Class|AkComponent|PostAssociatedAkEvent (Variables|Default|GetDeathScreamAK)))

(event Custom|Server_StopFlying
  (CallFunction|RPCStopFlying))

(event Custom|RPC_StartFlying
  (Class|AkComponent|PostAssociatedAkEvent (Variables|Default|GetFlightAK)))

(event Custom|OnDied
  (Collision|SetCollisionResponsetoChannel (Variables|Character|GetMesh) "ECC_Pawn" "ECR_Ignore")
  (Class|AkGameplayStatics|PostEvent "/Game/Audio/secLord_death.secLord_death" 0 false))

(event Custom|OnDamageTaken_Event_0
  (Class|AkComponent|PostAssociatedAkEvent (Variables|Default|GetHurtAK))
  (Components|Activation|Activate (Variables|Default|GetBlood) true)
  (Utilities|FlowControl|Delay 0.5)
  (Components|Activation|Deactivate (Variables|Default|GetBlood)))

(event Custom|StartFlying_Event
  (CallFunction|RPCStartFlying))

(event Custom|StopFlying_Event
  (Networking|SwitchHasAuthority
    (:Authority
      (CallFunction|RPCStopFlying))
    (:Remote
      (CallFunction|ServerStopFlying))))

(event Custom|Server_OnBossActive
  (CallFunction|RPConBossActive))

(event EventTick
  (params (DeltaSeconds :type Float%20%28single-precision%29)))

(event Collision|EventActorBeginOverlap
  (params (OtherActor :type Actor%20Object%20Reference)))

(event EventBeginPlay
  (EventDispatchers|AssignOnDied (Variables|Default|GetBP_BossDamageable) (delegate Custom|OnDied_Event_0))
  (Utilities|FlowControl|Sequence
    (:then_0
      (Rendering|SetActorHiddenInGame true)
      (Variables|Default|SetIsActive false)
      (Collision|SetCollisionResponsetoChannel (Variables|Character|GetMesh) "ECC_Pawn" "ECR_Overlap")
      (EventDispatchers|BindEventtoOnDied (Variables|Default|GetBP_BossDamageable) (delegate Custom|OnDied))
      (bind _returnvalue (Rendering|Material|CreateDynamicMaterialInstance (Variables|Character|GetMesh) 0 "/Game/Materials/Final_Materials/M_Boss_WeakPoint.M_Boss_WeakPoint" :!class /Script/Engine.PrimitiveComponent))
      (Variables|Default|SetWeakPointMaterial _returnvalue)
      (EventDispatchers|BindEventtoOnHealthChanged (Variables|Default|GetBP_BossDamageable) (delegate Custom|CustomEvent_0)))
    (:then_1
      (EventDispatchers|AssignOnDamageTaken (Variables|Default|GetBP_BossDamageable) (delegate Custom|OnDamageTaken_Event_0)))))

(fn ConstructionScript
  (bind _mesh (Variables|Character|GetMesh))
  (Utilities|FlowControl|Sequence
    (:then_0
      (Transformation|AttachComponentToComponent (Variables|Default|GetRigthAttackHitbox) (Variables|Character|GetMesh) "AttackSocketRight" "SnapToTarget" "SnapToTarget" "SnapToTarget" true)
      (Transformation|AttachComponentToComponent (Variables|Default|GetLeftAttackHitbox) (Variables|Character|GetMesh) "AttackSocketLeft" "SnapToTarget" "SnapToTarget" "SnapToTarget" true)
      (Transformation|AttachComponentToComponent (Variables|Default|GetEggSpawningContainer) (Variables|Character|GetMesh) "EggSpawnSocket" "SnapToTarget" "SnapToTarget" "SnapToTarget" true)
      (Transformation|AttachComponentToComponent (Variables|Default|GetWeakPointContainer) (Variables|Character|GetMesh) "WeakPointSocket" "SnapToTarget" "SnapToTarget" "SnapToTarget" true)
      (Transformation|AttachComponentToComponent (Variables|Default|GetScreamAK) (Variables|Character|GetMesh) "MouthSocket" "SnapToTarget" "SnapToTarget" "SnapToTarget" true))
    (:then_1
      (Transformation|AttachComponentToComponent (Variables|Default|GetRearLeftFootAK) _mesh "RearLeftFootSocket" "SnapToTarget" "SnapToTarget" "SnapToTarget" true))
    (:then_2
      (Transformation|AttachComponentToComponent (Variables|Default|GetRearRightFootAK) _mesh "RearRightFootSocket" "SnapToTarget" "SnapToTarget" "SnapToTarget" true))
    (:then_3
      (Transformation|AttachComponentToComponent (Variables|Default|GetFrontLeftFootAK) _mesh "FrontLeftFootSocket" "SnapToTarget" "SnapToTarget" "SnapToTarget" true))
    (:then_4
      (Transformation|AttachComponentToComponent (Variables|Default|GetFrontRightFootAK) _mesh "FrontRightFootSocket" "SnapToTarget" "SnapToTarget" "SnapToTarget" true))))

(fn ToggleDamage
  (params (CanDamage :type Boolean))
  (Utilities|FlowControl|Sequence
    (:then_0
      (Class|AttackHitbox|SetCanDamage (Variables|Default|GetRigthAttackHitbox) CanDamage))
    (:then_1
      (Class|AttackHitbox|SetCanDamage (Variables|Default|GetLeftAttackHitbox) CanDamage))))
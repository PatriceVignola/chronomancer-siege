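; BP_SoundManager is a Wwise music manager that switches between menu, exploration and fight music and controls gameplay music layers.
; On BeginPlay it gets an AkComponent attached to itself and caches it.
; Each custom event posts a single Ak event on that component, covering music start, the record and rewind layers, and death-rewind on and off.
; It keeps no playback state and does nothing on Tick.
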(event EventBeginPlay
  (bind _returnvalue (Class|AkGameplayStatics|GetAkComponent self "None" "0, 0, 0" "KeepRelativeOffset"))
  (Variables|Default|SetAkComponent _returnvalue))

(event EventTick
  (params (DeltaSeconds :type Float%20%28single-precision%29)))

(event EventOnRecordLayerRequested
  (Class|AkComponent|PostAkEvent (Variables|Default|GetAkComponent) "/Game/Audio/RecordOn.RecordOn"))

(event EventEnableMusic
  (Class|AkComponent|PostAkEvent (Variables|Default|GetAkComponent) "/Game/Audio/StartGame.StartGame"))

(event EventPlayMainMenuMusic
  (Class|AkComponent|PostAkEvent (Variables|Default|GetAkComponent) "/Game/Audio/MUS_Menu.MUS_Menu"))

(event EventOnRewindLayerRequested
  (Class|AkComponent|PostAkEvent (Variables|Default|GetAkComponent) "/Game/Audio/RewindOn.RewindOn"))

(event EventPlayExplorationMusic
  (Class|AkComponent|PostAkEvent (Variables|Default|GetAkComponent) "/Game/Audio/MUS_Explo.MUS_Explo"))

(event EventOnFightLayerRequested
  (Class|AkComponent|PostAkEvent (Variables|Default|GetAkComponent) "/Game/Audio/MUS_Fight.MUS_Fight"))

(event EventOnPlayDeathRewindLayerRequested
  (Class|AkComponent|PostAkEvent (Variables|Default|GetAkComponent) "/Game/Audio/RewindDeathON.RewindDeathON"))

(event EventOnStopDeathRewindLayerRequested
  (Class|AkComponent|PostAkEvent (Variables|Default|GetAkComponent) "/Game/Audio/RewindDeathOff.RewindDeathOff"))
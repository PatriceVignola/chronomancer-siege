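; BP_Elevator is an activable elevator that animates and plays sound when open or close is requested.
; Open and close requests toggle the Elevator flag on its AnimBP_Elevator1 anim instance and post the ActivationAK Wwise event.
; Pillar activated, active and deactivated events swap a mesh material slot to show pillar state.
; The construction script snaps the audio component to the moving floor socket so sound follows the platform.
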(event Custom|OnOpenActivableRequested_Event_0
  (bind _asanim_bp_elevator_1 (Utilities|Casting|CastToAnimBP_Elevator1 (Components|SkeletalMesh|GetAnimInstance (Variables|Character|GetMesh))))
  (Variables|/Game/Models/AnimatedObjects/AnimBP_Elevator1.AnimBP_Elevator1_C|SetElevator _asanim_bp_elevator_1 false)
  (Class|AkComponent|PostAssociatedAkEvent (Variables|Default|GetActivationAK)))

(event Custom|OnCloseActivableRequested_Event_0
  (bind _asanim_bp_elevator_1 (Utilities|Casting|CastToAnimBP_Elevator1 (Components|SkeletalMesh|GetAnimInstance (Variables|Character|GetMesh))))
  (Variables|/Game/Models/AnimatedObjects/AnimBP_Elevator1.AnimBP_Elevator1_C|SetElevator _asanim_bp_elevator_1 true)
  (Class|AkComponent|PostAssociatedAkEvent (Variables|Default|GetActivationAK)))

(event Custom|PillardActive
  (Rendering|Material|SetMaterial (Variables|Character|GetMesh) 1 "/Game/Materials/Final_Materials/Pillard-Active.Pillard-Active"))

(event Custom|PillardActivated
  (Rendering|Material|SetMaterial (Variables|Character|GetMesh) 1 "/Game/Materials/Final_Materials/Pillard-Activated.Pillard-Activated"))

(event Custom|PillardDeactivated
  (Rendering|Material|SetMaterial (Variables|Character|GetMesh) 1 "/Game/Materials/Final_Materials/Pillard-Desactivated.Pillard-Desactivated"))

(event EventBeginPlay
  (EventDispatchers|AssignOnOpenActivableRequested (delegate Custom|OnOpenActivableRequested_Event_0))
  (EventDispatchers|AssignOnCloseActivableRequested (delegate Custom|OnCloseActivableRequested_Event_0))
  (EventDispatchers|BindEventtoOnPillarActivated (delegate Custom|PillardActivated))
  (EventDispatchers|BindEventtoOnPillarActive (delegate Custom|PillardActive))
  (EventDispatchers|BindEventtoOnPillarDeactivated (delegate Custom|PillardDeactivated)))

(event Collision|EventActorBeginOverlap
  (params (OtherActor :type Actor%20Object%20Reference)))

(event EventTick
  (params (DeltaSeconds :type Float%20%28single-precision%29)))

(fn ConstructionScript
  (Transformation|AttachComponentToComponent (Variables|Default|GetActivationAK) (Variables|Character|GetMesh) "MoveableFloorSocket" "SnapToTarget" "SnapToTarget" "SnapToTarget" true))
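; Player controller for Chronomancer Siege that handles character selection input: focusing Warrior or Mage, selecting and unselecting.
; Axis inputs past a threshold change focus, and button presses select or unselect.
; Each input branches on authority: the host calls the OnServer variant, while a remote client sends a Server RPC that calls the cached GameState's OnClient variant, keeping host and client choices separate.
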(event Custom|Server_CallOnFocusMageOnClient
  (Default|CallOnFocusMageonClient (Variables|Default|GetGameState)))

(event Custom|Server_CallOnFocusWarriorOnClient
  (Default|CallOnFocusWarrioronClient (Variables|Default|GetGameState)))

(event Custom|Server_CallOnSelectCharacterOnClient
  (Default|CallOnSelectCharacteronClient (Variables|Default|GetGameState)))

(event Custom|Server_CallOnUnselectCharacterOnClient
  (Default|CallOnUnselectCharacteronClient (Variables|Default|GetGameState)))

(event EventBeginPlay
  (bind _asbp_chronomancer_siege_game_state (Utilities|Casting|CastToBP_ChronomancerSiegeGameState (Game|GetGameState)))
  (Variables|Default|SetGameState _asbp_chronomancer_siege_game_state))

(event EventTick
  (params (DeltaSeconds :type Float%20%28single-precision%29)))

(event Input|ActionEvents|InputActionUnselectMenuOption
  (params (Key :type Key%20Structure :default "AnyKey"))
  (:Pressed
    (Networking|SwitchHasAuthority
      (:Authority
        (Default|CallOnUnselectCharacteronServer))
      (:Remote
        (CallFunction|ServerCallonUnselectCharacteronClient)))))

(event Input|ActionEvents|InputActionSelectMenuOption
  (params (Key :type Key%20Structure :default "AnyKey"))
  (:Pressed
    (Networking|SwitchHasAuthority
      (:Authority
        (Default|CallOnSelectCharacteronServer))
      (:Remote
        (CallFunction|ServerCallonSelectCharacteronClient)))))

(event Input|AxisEvents|InputAxisFocusPrevOption
  (params (AxisValue :type Float%20%28single-precision%29))
  (if (> AxisValue 0.9)
    (Networking|SwitchHasAuthority
      (:Authority
        (Default|CallOnFocusWarrioronServer))
      (:Remote
        (CallFunction|ServerCallonFocusWarrioronClient)))))

(event Input|AxisEvents|InputAxisFocusNextOption
  (params (AxisValue :type Float%20%28single-precision%29))
  (if (> AxisValue 0.9)
    (Networking|SwitchHasAuthority
      (:Authority
        (Default|CallOnFocusMageonServer))
      (:Remote
        (CallFunction|ServerCallonFocusMageonClient)))))

(fn ConstructionScript)
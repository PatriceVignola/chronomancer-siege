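; Runs the two-player Warrior/Mage character select, from LAN matchmaking to game start.
; The host searches LAN sessions at random delays, dropping its session to join an open one, until two players connect.
; Controller and GameState dispatchers drive focus, select and lock handlers for server and client, with RPCs updating the remote UI.
; Once both pick, the server triggers loading screens, streams the temple level and notifies the GameMode of character assignment.
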(event Custom|RefreshSearchPlayer
  (bind _returnvalue (Game|GetPlayerController 0))
  (if (not (Variables|Default|GetPlayersConnected))
    (Utilities|FlowControl|Delay (* (Math|Random|RandomFloat) 1e+01))
    (bind _results (|FindSessions (Game|GetPlayerController 0) 0 true)
      (:OnSuccess
        (Development|PrintString (Utilities|String|ToString(Integer) (Utilities|Array|Length _results)))
        (if (== (Utilities|Array|Length _results) 0)
          (CallFunction|RefreshSearchPlayer)
          (else
            (bind _array_element (Utilities|Array|ForEachLoopwithBreak _results :!label _label)
              (:LoopBody
                (if (and (< (Class|FindSessionsCallbackProxy|GetCurrentPlayers _array_element) (Class|FindSessionsCallbackProxy|GetMaxPlayers _array_element)) (not (Variables|Default|GetPlayersConnected)))
                  (|DestroySession _returnvalue
                    (:OnSuccess
                      _)
                    (:OnFailure
                      _))
                  (|JoinSession _returnvalue _array_element
                    (:OnSuccess
                      (Variables|Default|SetGameJoined true)
                      (Development|PrintString "Game joined!")
                      (goto _label Break))
                    (:OnFailure
                      _))
                  (else
                    (Development|PrintString "NOT ENOUGH ROOM!!!!!!!!!!!!")))
                (CallFunction|RefreshSearchPlayer))
              (:Completed
                (if (not (Variables|Default|GetGameJoined))
                  (CallFunction|RefreshSearchPlayer)))))))
      (:OnFailure
        (CallFunction|RefreshSearchPlayer)))))

(event Custom|RPC_UnlockWarrior
  (Networking|SwitchHasAuthority
    (:Remote
      (CallFunction|UnlockWarrior))))

(event Custom|RPC_UnlockMage
  (Networking|SwitchHasAuthority
    (:Remote
      (CallFunction|UnlockMage))))

(event Custom|OnSelectCharacterOnServer_Event_0
  (CallFunction|HandleSelectCharacteronServer))

(event Custom|ShowWarriorLoadingScreen
  (bind _loadingscreenfadeduration (Variables|Default|GetLoadingScreenFadeDuration))
  (bind _returnvalue (UserInterface|CreateWidget "/Game/UI/UMG_WarriorLoadingScreen.UMG_WarriorLoadingScreen_C" (Variables|Default|GetController)))
  (bind _output_get (Variables|Default|SetWarriorLoadingUI _returnvalue))
  (UserInterface|Viewport|AddtoViewport _output_get 10)
  (Default|Fadein _output_get _loadingscreenfadeduration)
  (Utilities|FlowControl|Delay _loadingscreenfadeduration))

(event Custom|OnUnselectCharacterOnServer_Event_0
  (CallFunction|HandleUnselectCharacteronServer))

(event Custom|RPC_SelectWarrior
  (Networking|SwitchHasAuthority
    (:Remote
      (CallFunction|SelectWarrior))))

(event Custom|RPC_SelectMage
  (Networking|SwitchHasAuthority
    (:Remote
      (CallFunction|SelectMage))))

(event Custom|ShowMageLoadingScreen
  (bind _loadingscreenfadeduration (Variables|Default|GetLoadingScreenFadeDuration))
  (bind _returnvalue (UserInterface|CreateWidget "/Game/UI/UMG_MageLoadingScreen.UMG_MageLoadingScreen_C" (Variables|Default|GetController)))
  (bind _output_get (Variables|Default|SetMageLoadingUI _returnvalue))
  (UserInterface|Viewport|AddtoViewport _output_get 10)
  (Default|Fadein _output_get _loadingscreenfadeduration)
  (Utilities|FlowControl|Delay _loadingscreenfadeduration))

(event Custom|StartGame
  (Networking|SwitchHasAuthority
    (:Authority
      (Variables|Default|SetGameStarting true)
      (Utilities|FlowControl|Delay 2.0)
      (switch Utilities|FlowControl|Switch|SwitchonCharacterTypeEnum (Variables|Default|GetServerSelectedCharacter)
        (:NewEnumerator1
          (CallFunction|ShowWarriorLoadingScreen)
          (CallFunction|RPCShowMageLoadingScreen))
        (:NewEnumerator2
          (CallFunction|ShowMageLoadingScreen)
          (CallFunction|RPCShowWarriorLoadingScreen)))
      (Utilities|FlowControl|Delay (Variables|Default|GetLoadingScreenFadeDuration))
      (Game|LoadStreamLevel(byName) "/Game/Levels/00101_CenturianMineTemple" true)
      (Utilities|FlowControl|Delay 3.0)
      (bind _asbp_academia_2017game_mode (Utilities|Casting|CastToBP_Academia2017GameMode (Game|GetGameMode)))
      (switch Utilities|FlowControl|Switch|SwitchonCharacterTypeEnum (Variables|Default|GetServerSelectedCharacter)
        (:NewEnumerator1
          (Class|Academia2017GameMode|NotifyLevelStreamed _asbp_academia_2017game_mode (Utilities|Array|MakeArray 0 1)))
        (:NewEnumerator2
          (Class|Academia2017GameMode|NotifyLevelStreamed _asbp_academia_2017game_mode (Utilities|Array|MakeArray 1 0))))
      (Utilities|FlowControl|Delay 5.0)
      (CallFunction|RPCRemoveUI))))

(event Custom|RPC_RemoveUI
  (bind _loadingscreenfadeduration (Variables|Default|GetLoadingScreenFadeDuration))
  (bind _warriorloadingui (Variables|Default|GetWarriorLoadingUI))
  (bind _loadingscreenfadeduration_2 (Variables|Default|GetLoadingScreenFadeDuration))
  (bind _mageloadingui (Variables|Default|GetMageLoadingUI))
  (Widget|RemovefromParent (Variables|Default|GetCharacterSelectUI))
  (if (Utilities|IsValid _warriorloadingui)
    (Default|FadeOut _warriorloadingui _loadingscreenfadeduration)
    (Utilities|FlowControl|Delay _loadingscreenfadeduration)
    (Widget|RemovefromParent _warriorloadingui))
  (if (Utilities|IsValid _mageloadingui)
    (Default|FadeOut _mageloadingui _loadingscreenfadeduration_2)
    (Utilities|FlowControl|Delay _loadingscreenfadeduration_2)
    (Widget|RemovefromParent _mageloadingui))
  (bind _asbp_academia_2017game_mode (Utilities|Casting|CastToBP_Academia2017GameMode (Game|GetGameMode)))
  (Default|CallOnLevelVisuallyFinishedStreaming _asbp_academia_2017game_mode)
  (bind _asbp_academia_2017game_mode_2 (Utilities|Casting|CastToBP_Academia2017GameMode (Game|GetGameMode)))
  (Class|Academia2017GameMode|ReEnableInput _asbp_academia_2017game_mode_2)
  (Game|UnloadStreamLevel(byName) "/Game/Levels/CharacterSelection"))

(event Custom|StartSearching
  (params (NewParam :type BP%20Network%20Manager%20Object%20Reference))
  (bind _gamestate (Variables|Default|GetGameState))
  (Variables|Default|SetNetworkManager NewParam)
  (CallFunction|AddCharacterSelectUI)
  (CallFunction|HandleFocusWarrioronClient)
  (Variables|Default|SetClientFocusedCharacter "NewEnumerator1")
  (Variables|Default|SetSearchingForPlayers false)
  (bind _asbp_chronomancer_siege_controller (Utilities|Casting|CastToBP_ChronomancerSiegeController (Game|GetPlayerController 0)))
  (bind _output_get (Variables|Default|SetController _asbp_chronomancer_siege_controller))
  (EventDispatchers|AssignOnFocusWarrioronClient (Variables|Default|GetGameState) (delegate Custom|OnFocusWarriorOnClient_Event_1))
  (EventDispatchers|AssignOnFocusWarrioronServer _output_get (delegate Custom|OnFocusWarriorOnServer_Event_0))
  (EventDispatchers|AssignOnFocusMageonClient (Variables|Default|GetGameState) (delegate Custom|OnFocusMageOnClient_Event_0))
  (EventDispatchers|AssignOnFocusMageonServer _output_get (delegate Custom|OnFocusMageOnServer_Event_0))
  (EventDispatchers|AssignOnSelectCharacteronClient _gamestate (delegate Custom|OnSelectCharacterOnClient_Event_0))
  (EventDispatchers|AssignOnUnselectCharacteronClient _gamestate (delegate Custom|OnUnselectCharacterOnClient_Event_0))
  (EventDispatchers|AssignOnSelectCharacteronServer _output_get (delegate Custom|OnSelectCharacterOnServer_Event_0))
  (EventDispatchers|AssignOnUnselectCharacteronServer _output_get (delegate Custom|OnUnselectCharacterOnServer_Event_0))
  (Utilities|FlowControl|Sequence
    (:then_0
      (Networking|SwitchHasAuthority
        (:Authority
          (if (not (Variables|Default|GetPlayersConnected))
            (CallFunction|RefreshSearchPlayer)))
        (:Remote
          (Variables|Default|SetPlayersConnected true)
          (CallFunction|StopSearching)
          (CallFunction|FocusMage)
          (Variables|Default|SetClientFocusedCharacter "NewEnumerator2"))))
    (:then_1
      (EventDispatchers|AssignOnClientJoined (Variables|Default|GetNetworkManager) (delegate Custom|OnClientJoined_Event_0)))
    (:then_2
      (Networking|SwitchHasAuthority
        (:Authority
          (if (== (Utilities|Array|Length (Variables|/Script/Engine.GameStateBase|GetPlayerArray (Game|GetGameState))) 2)
            (CallFunction|StopSearching)
            (CallFunction|HandleFocusWarrioronServer)))))))

(event Custom|OnFocusWarriorOnClient_Event_1
  (CallFunction|HandleFocusWarrioronClient))

(event Custom|OnFocusMageOnClient_Event_0
  (CallFunction|HandleFocusMageonClient))

(event Custom|OnSelectCharacterOnClient_Event_0
  (CallFunction|HandleSelectCharacteronClient))

(event Custom|OnUnselectCharacterOnClient_Event_0
  (CallFunction|HandleUnselectCharacteronClient))

(event Custom|OnFocusWarriorOnServer_Event_0
  (CallFunction|HandleFocusWarrioronServer))

(event Custom|OnClientJoined_Event_0
  (Networking|SwitchHasAuthority
    (:Authority
      (if (== (Utilities|Array|Length (Variables|/Script/Engine.GameStateBase|GetPlayerArray (Game|GetGameState))) 2)
        (Variables|Default|SetPlayersConnected true)
        (CallFunction|StopSearching)
        (CallFunction|HandleFocusWarrioronServer)
        (CallFunction|HandleFocusMageonClient)
        (Variables|Default|SetServerFocusedCharacter "NewEnumerator1")
        (Variables|Default|SetClientFocusedCharacter "NewEnumerator2")))))

(event Custom|RPC_ShowWarriorLoadingScreen
  (bind _returnvalue (Game|GetGameState))
  (bind _returnvalue_2 (Actor|GetComponentbyClass _returnvalue "/Game/Blueprints/BP_SoundManager.BP_SoundManager_C"))
  (Class|SoundManagerComponent|EnableMusic _returnvalue_2)
  (Class|SoundManagerComponent|PlayExplorationMusic _returnvalue_2)
  (Networking|SwitchHasAuthority
    (:Remote
      (CallFunction|ShowWarriorLoadingScreen))))

(event Custom|RPC_LockWarrior
  (params (ShouldRefocus :type Boolean))
  (Networking|SwitchHasAuthority
    (:Remote
      (CallFunction|LockWarrior)
      (if ShouldRefocus
        (CallFunction|FocusMage)))))

(event Custom|RPC_LockMage
  (params (ShouldRefocus :type Boolean))
  (Networking|SwitchHasAuthority
    (:Remote
      (CallFunction|LockMage)
      (if ShouldRefocus
        (CallFunction|FocusWarrior)))))

(event Custom|RPC_ShowMageLoadingScreen
  (bind _returnvalue (Game|GetGameState))
  (bind _returnvalue_2 (Actor|GetComponentbyClass _returnvalue "/Game/Blueprints/BP_SoundManager.BP_SoundManager_C"))
  (Class|SoundManagerComponent|EnableMusic _returnvalue_2)
  (Class|SoundManagerComponent|PlayExplorationMusic _returnvalue_2)
  (Networking|SwitchHasAuthority
    (:Remote
      (CallFunction|ShowMageLoadingScreen))))

(event Custom|OnFocusMageOnServer_Event_0
  (CallFunction|HandleFocusMageonServer))

(event Custom|RPC_FocusWarrior
  (Networking|SwitchHasAuthority
    (:Remote
      (CallFunction|FocusWarrior))))

(event Custom|RPC_FocusMage
  (Networking|SwitchHasAuthority
    (:Remote
      (CallFunction|FocusMage))))

(event EventBeginPlay
  (bind _asbp_chronomancer_siege_game_state (Utilities|Casting|CastToBP_ChronomancerSiegeGameState (Game|GetGameState)))
  (Variables|Default|SetGameState _asbp_chronomancer_siege_game_state))

(fn ConstructionScript)

(fn AddCharacterSelectUI
  (bind _returnvalue (UserInterface|CreateWidget "/Game/UI/UMG_CharacterSelect.UMG_CharacterSelect_C" (Game|GetPlayerController 0)))
  (bind _output_get (Variables|Default|SetCharacterSelectUI _returnvalue))
  (UserInterface|Viewport|AddtoViewport _output_get 0))

(fn FocusWarrior
  (bind _characterselectui (Variables|Default|GetCharacterSelectUI))
  (Widget|SetVisibility (Variables|/Game/UI/UMG_CharacterSelect.UMG_CharacterSelect_C|GetFocusedWarriorImage _characterselectui) "Visible")
  (Widget|SetVisibility (Variables|/Game/UI/UMG_CharacterSelect.UMG_CharacterSelect_C|GetFocusedMageImage _characterselectui) "Hidden")
  (Widget|SetVisibility (Variables|/Game/UI/UMG_CharacterSelect.UMG_CharacterSelect_C|GetSelectedWarriorImage _characterselectui) "Hidden"))

(fn HandleFocusWarrioronClient
  (bind _asbp_academia_2017game_mode (Utilities|Casting|CastToBP_Academia2017GameMode (Game|GetGameMode))
    (:then
      (if (Variables|/Game/Blueprints/BP_Academia2017GameMode.BP_Academia2017GameMode_C|GetWarriorServerForced _asbp_academia_2017game_mode)
        (CallFunction|HandleFocusMageonClient)
        (else
          (if (not (Math|Boolean|ORBoolean (Variables|Default|GetGameStarting) (Variables|Default|GetSearchingForPlayers) (not (Variables|Default|GetPlayersConnected)))) :!label _label
            (switch Utilities|FlowControl|Switch|SwitchonCharacterTypeEnum (Variables|Default|GetServerSelectedCharacter)
              (:NewEnumerator0
                _)
              (:NewEnumerator2
                _))
            (switch Utilities|FlowControl|Switch|SwitchonCharacterTypeEnum (Variables|Default|GetClientSelectedCharacter)
              (:NewEnumerator0
                (switch Utilities|FlowControl|Switch|SwitchonCharacterTypeEnum (Variables|Default|GetClientFocusedCharacter)
                  (:NewEnumerator0
                    _)
                  (:NewEnumerator2
                    _))
                (Variables|Default|SetClientFocusedCharacter "NewEnumerator1")
                (CallFunction|RPCFocusWarrior)))))))
    (:CastFailed
      (goto _label))))

(fn HandleFocusWarrioronServer
  (if (not (Math|Boolean|ORBoolean (Variables|Default|GetGameStarting) (Variables|Default|GetSearchingForPlayers) (not (Variables|Default|GetPlayersConnected))))
    (switch Utilities|FlowControl|Switch|SwitchonCharacterTypeEnum (Variables|Default|GetClientSelectedCharacter)
      (:NewEnumerator0
        _)
      (:NewEnumerator2
        _))
    (switch Utilities|FlowControl|Switch|SwitchonCharacterTypeEnum (Variables|Default|GetServerSelectedCharacter)
      (:NewEnumerator0
        (switch Utilities|FlowControl|Switch|SwitchonCharacterTypeEnum (Variables|Default|GetServerFocusedCharacter)
          (:NewEnumerator0
            _)
          (:NewEnumerator2
            _))
        (Variables|Default|SetServerFocusedCharacter "NewEnumerator1")
        (CallFunction|FocusWarrior)))))

(fn HandleFocusMageonClient
  (if (not (Math|Boolean|ORBoolean (Variables|Default|GetGameStarting) (Variables|Default|GetSearchingForPlayers) (not (Variables|Default|GetPlayersConnected))))
    (switch Utilities|FlowControl|Switch|SwitchonCharacterTypeEnum (Variables|Default|GetServerSelectedCharacter)
      (:NewEnumerator0
        _)
      (:NewEnumerator1
        _))
    (switch Utilities|FlowControl|Switch|SwitchonCharacterTypeEnum (Variables|Default|GetClientSelectedCharacter)
      (:NewEnumerator0
        (switch Utilities|FlowControl|Switch|SwitchonCharacterTypeEnum (Variables|Default|GetClientFocusedCharacter)
          (:NewEnumerator0
            _)
          (:NewEnumerator1
            _))
        (Variables|Default|SetClientFocusedCharacter "NewEnumerator2")
        (CallFunction|RPCFocusMage)))))

(fn HandleFocusMageonServer
  (bind _asbp_academia_2017game_mode (Utilities|Casting|CastToBP_Academia2017GameMode (Game|GetGameMode))
    (:then
      (if (not (Variables|/Game/Blueprints/BP_Academia2017GameMode.BP_Academia2017GameMode_C|GetWarriorServerForced _asbp_academia_2017game_mode))
        (if (not (Math|Boolean|ORBoolean (Variables|Default|GetGameStarting) (Variables|Default|GetSearchingForPlayers) (not (Variables|Default|GetPlayersConnected)))) :!label _label
          (switch Utilities|FlowControl|Switch|SwitchonCharacterTypeEnum (Variables|Default|GetClientSelectedCharacter)
            (:NewEnumerator0
              _)
            (:NewEnumerator1
              _))
          (switch Utilities|FlowControl|Switch|SwitchonCharacterTypeEnum (Variables|Default|GetServerSelectedCharacter)
            (:NewEnumerator0
              (switch Utilities|FlowControl|Switch|SwitchonCharacterTypeEnum (Variables|Default|GetServerFocusedCharacter)
                (:NewEnumerator0
                  _)
                (:NewEnumerator1
                  _))
              (CallFunction|FocusMage)
              (Variables|Default|SetServerFocusedCharacter "NewEnumerator2"))))))
    (:CastFailed
      (goto _label))))

(fn FocusMage
  (bind _characterselectui (Variables|Default|GetCharacterSelectUI))
  (Widget|SetVisibility (Variables|/Game/UI/UMG_CharacterSelect.UMG_CharacterSelect_C|GetFocusedMageImage _characterselectui) "Visible")
  (Widget|SetVisibility (Variables|/Game/UI/UMG_CharacterSelect.UMG_CharacterSelect_C|GetFocusedWarriorImage _characterselectui) "Hidden")
  (Widget|SetVisibility (Variables|/Game/UI/UMG_CharacterSelect.UMG_CharacterSelect_C|GetSelectedMageImage _characterselectui) "Hidden"))

(fn HandleSelectCharacteronClient
  (if (not (Math|Boolean|ORBoolean (Variables|Default|GetGameStarting) (Variables|Default|GetSearchingForPlayers) (not (Variables|Default|GetPlayersConnected))))
    (switch Utilities|FlowControl|Switch|SwitchonCharacterTypeEnum (Variables|Default|GetClientSelectedCharacter)
      (:NewEnumerator0
        (switch Utilities|FlowControl|Switch|SwitchonCharacterTypeEnum (Variables|Default|GetClientFocusedCharacter)
          (:NewEnumerator1
            (CallFunction|RPCSelectWarrior)
            (Variables|Default|SetClientSelectedCharacter "NewEnumerator1")
            (CallFunction|LockWarrior)
            (switch Utilities|FlowControl|Switch|SwitchonCharacterTypeEnum (Variables|Default|GetServerSelectedCharacter)
              (:NewEnumerator0
                (CallFunction|FocusMage)
                (Variables|Default|SetServerFocusedCharacter "NewEnumerator2"))
              (:NewEnumerator1
                (CallFunction|StartGame :!label _label))
              (:NewEnumerator2
                (goto _label))))
          (:NewEnumerator2
            (CallFunction|RPCSelectMage)
            (Variables|Default|SetClientSelectedCharacter "NewEnumerator2")
            (CallFunction|LockMage)
            (switch Utilities|FlowControl|Switch|SwitchonCharacterTypeEnum (Variables|Default|GetServerSelectedCharacter)
              (:NewEnumerator0
                (CallFunction|FocusWarrior)
                (Variables|Default|SetServerFocusedCharacter "NewEnumerator1"))
              (:NewEnumerator1
                (goto _label))
              (:NewEnumerator2
                (goto _label)))))))))

(fn HandleUnselectCharacteronClient
  (if (not (Math|Boolean|ORBoolean (Variables|Default|GetGameStarting) (Variables|Default|GetSearchingForPlayers) (not (Variables|Default|GetPlayersConnected))))
    (switch Utilities|FlowControl|Switch|SwitchonCharacterTypeEnum (Variables|Default|GetClientSelectedCharacter)
      (:NewEnumerator1
        (CallFunction|RPCFocusWarrior)
        (CallFunction|UnlockWarrior)
        (Variables|Default|SetClientFocusedCharacter "NewEnumerator1"))
      (:NewEnumerator2
        (CallFunction|RPCFocusMage)
        (CallFunction|UnlockMage)
        (Variables|Default|SetClientFocusedCharacter "NewEnumerator2")))
    (Variables|Default|SetClientSelectedCharacter "NewEnumerator0")))

(fn HandleSelectCharacteronServer
  (if (not (Math|Boolean|ORBoolean (Variables|Default|GetGameStarting) (Variables|Default|GetSearchingForPlayers) (not (Variables|Default|GetPlayersConnected))))
    (switch Utilities|FlowControl|Switch|SwitchonCharacterTypeEnum (Variables|Default|GetServerSelectedCharacter)
      (:NewEnumerator0
        (switch Utilities|FlowControl|Switch|SwitchonCharacterTypeEnum (Variables|Default|GetServerFocusedCharacter)
          (:NewEnumerator1
            (CallFunction|SelectWarrior)
            (Variables|Default|SetServerSelectedCharacter "NewEnumerator1")
            (switch Utilities|FlowControl|Switch|SwitchonCharacterTypeEnum (Variables|Default|GetClientSelectedCharacter)
              (:NewEnumerator0
                (CallFunction|RPCLockWarrior true)
                (Variables|Default|SetClientFocusedCharacter "NewEnumerator2"))
              (:NewEnumerator1
                (CallFunction|RPCLockWarrior false :!label _label)
                (CallFunction|StartGame :!label _label_2))
              (:NewEnumerator2
                (goto _label))))
          (:NewEnumerator2
            (CallFunction|SelectMage)
            (Variables|Default|SetServerSelectedCharacter "NewEnumerator2")
            (switch Utilities|FlowControl|Switch|SwitchonCharacterTypeEnum (Variables|Default|GetClientSelectedCharacter)
              (:NewEnumerator0
                (CallFunction|RPCLockMage true)
                (Variables|Default|SetClientFocusedCharacter "NewEnumerator1"))
              (:NewEnumerator1
                (CallFunction|RPCLockMage false :!label _label_3)
                (goto _label_2))
              (:NewEnumerator2
                (goto _label_3)))))))))

(fn HandleUnselectCharacteronServer
  (if (not (Math|Boolean|ORBoolean (Variables|Default|GetGameStarting) (Variables|Default|GetSearchingForPlayers) (not (Variables|Default|GetPlayersConnected))))
    (switch Utilities|FlowControl|Switch|SwitchonCharacterTypeEnum (Variables|Default|GetServerSelectedCharacter)
      (:NewEnumerator1
        (CallFunction|FocusWarrior)
        (Variables|Default|SetServerFocusedCharacter "NewEnumerator1")
        (CallFunction|RPCUnlockWarrior))
      (:NewEnumerator2
        (CallFunction|FocusMage)
        (Variables|Default|SetServerFocusedCharacter "NewEnumerator2")
        (CallFunction|RPCUnlockMage)))
    (Variables|Default|SetServerSelectedCharacter "NewEnumerator0")))

(fn SelectWarrior
  (bind _characterselectui (Variables|Default|GetCharacterSelectUI))
  (Widget|SetVisibility (Variables|/Game/UI/UMG_CharacterSelect.UMG_CharacterSelect_C|GetSelectedWarriorImage _characterselectui) "Visible")
  (Widget|SetVisibility (Variables|/Game/UI/UMG_CharacterSelect.UMG_CharacterSelect_C|GetFocusedWarriorImage _characterselectui) "Hidden"))

(fn SelectMage
  (bind _characterselectui (Variables|Default|GetCharacterSelectUI))
  (Widget|SetVisibility (Variables|/Game/UI/UMG_CharacterSelect.UMG_CharacterSelect_C|GetSelectedMageImage _characterselectui) "Visible")
  (Widget|SetVisibility (Variables|/Game/UI/UMG_CharacterSelect.UMG_CharacterSelect_C|GetFocusedMageImage _characterselectui) "Hidden"))

(fn LockWarrior
  (bind _characterselectui (Variables|Default|GetCharacterSelectUI))
  (Widget|SetVisibility (Variables|/Game/UI/UMG_CharacterSelect.UMG_CharacterSelect_C|GetLockedWarriorImage _characterselectui) "Visible")
  (Widget|SetVisibility (Variables|/Game/UI/UMG_CharacterSelect.UMG_CharacterSelect_C|GetFocusedWarriorImage _characterselectui) "Hidden"))

(fn LockMage
  (bind _characterselectui (Variables|Default|GetCharacterSelectUI))
  (Widget|SetVisibility (Variables|/Game/UI/UMG_CharacterSelect.UMG_CharacterSelect_C|GetLockedMageImage _characterselectui) "Visible")
  (Widget|SetVisibility (Variables|/Game/UI/UMG_CharacterSelect.UMG_CharacterSelect_C|GetFocusedMageImage _characterselectui) "Hidden"))

(fn UnlockWarrior
  (Widget|SetVisibility (Variables|/Game/UI/UMG_CharacterSelect.UMG_CharacterSelect_C|GetLockedWarriorImage (Variables|Default|GetCharacterSelectUI)) "Hidden"))

(fn UnlockMage
  (Widget|SetVisibility (Variables|/Game/UI/UMG_CharacterSelect.UMG_CharacterSelect_C|GetLockedMageImage (Variables|Default|GetCharacterSelectUI)) "Hidden"))

(fn StopSearching
  (bind _characterselectui (Variables|Default|GetCharacterSelectUI))
  (Variables|Default|SetSearchingForPlayers false)
  (Widget|SetVisibility (Variables|/Game/UI/UMG_CharacterSelect.UMG_CharacterSelect_C|GetscanningMag _characterselectui) "Hidden")
  (Widget|SetVisibility (Variables|/Game/UI/UMG_CharacterSelect.UMG_CharacterSelect_C|GetscanningWarrior _characterselectui) "Hidden"))
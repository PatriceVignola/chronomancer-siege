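; BP_WarriorClone is a warrior clone actor that adds Wwise audio to replayed clone actions.
; The construction script snaps the ghost sound emitter to the sword socket and the footstep emitters to the foot sockets.
; On BeginPlay it starts the ghost sound and binds to ReplayableBones events for attacks and left and right footsteps.
; Attack events pick a sound by attack type index, while footsteps post each emitter's own event.
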(event Custom|OnCloneAttackStarted_Event_1
  (params (AttackType :type Integer))
  (if (< AttackType (Utilities|Array|Length (Variables|Default|GetAttackSounds)))
    (Class|AkComponent|PostAkEvent (Variables|Default|GetAttackAK) (Utilities|Array|Get(acopy) (Variables|Default|GetAttackSounds) AttackType))))

(event Custom|OnCloneRightFootstepPlayed_Event_0
  (Class|AkComponent|PostAssociatedAkEvent (Variables|Default|GetRightFootAK)))

(event Custom|OnCloneLeftFootstepPlayed_Event_0
  (Class|AkComponent|PostAssociatedAkEvent (Variables|Default|GetLeftFootAK)))

(event EventTick
  (params (DeltaSeconds :type Float%20%28single-precision%29)))

(event EventBeginPlay
  (bind _replayablebones (Variables|Default|GetReplayableBones))
  (Utilities|FlowControl|Sequence
    (:then_0
      (EventDispatchers|AssignOnCloneAttackStarted (Variables|Default|GetReplayableBones) (delegate Custom|OnCloneAttackStarted_Event_1))
      (Class|AkComponent|PostAssociatedAkEvent (Variables|Default|GetGhostAK)))
    (:then_1
      (EventDispatchers|AssignOnCloneLeftFootstepPlayed _replayablebones (delegate Custom|OnCloneLeftFootstepPlayed_Event_0))
      (EventDispatchers|AssignOnCloneRightFootstepPlayed _replayablebones (delegate Custom|OnCloneRightFootstepPlayed_Event_0)))))

(fn ConstructionScript
  (Utilities|FlowControl|Sequence
    (:then_0
      (Transformation|AttachComponentToComponent (Variables|Default|GetGhostAK) (Variables|Character|GetMesh) "SwordSocket" "SnapToTarget" "SnapToTarget" "SnapToTarget" true))
    (:then_1
      (Transformation|AttachComponentToComponent (Variables|Default|GetLeftFootAK) (Variables|Character|GetMesh) "LeftFootSocket" "SnapToTarget" "SnapToTarget" "SnapToTarget" true))
    (:then_2
      (Transformation|AttachComponentToComponent (Variables|Default|GetRightFootAK) (Variables|Character|GetMesh) "RightFootSocket" "SnapToTarget" "SnapToTarget" "SnapToTarget" true))))
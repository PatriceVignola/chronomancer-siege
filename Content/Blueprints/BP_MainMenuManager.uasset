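; Main menu manager actor for a two-player LAN co-op game, where players pick Warrior to host or Mage to join.
; It creates the menu widget, maps axis and action inputs to focus, select and unselect, and toggles hero images and loading indicators.
; Warrior opens a listen-server level; Mage repeatedly searches for open sessions.
; When two players are present, the authority stream-loads the mine temple level and removes the menu.
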(event Custom|RefreshCreateGame
  (|Session (Game|GetPlayerController 0) 2 true
    (:OnSuccess
      (Development|PrintString "Game created!")
      (Game|OpenLevel(byName) "Persistant" true "listen"))
    (:OnFailure
      (CallFunction|RefreshCreateGame))))

(event Custom|RemoveMainMenuUI
  (Widget|RemovefromParent (Variables|Default|GetMainMenuUI))
  (Game|UnloadStreamLevel(byName) "/Game/Levels/MainMenu"))

(event Custom|RefreshJoinGame
  (bind _returnvalue (Game|GetPlayerController 0))
  (Development|PrintString "Refreshing games...")
  (bind _results (|FindSessions (Game|GetPlayerController 0) 0 true)
    (:OnSuccess
      (if (Variables|Default|GetHeroSelected)
        (if (== (Utilities|Array|Length _results) 0)
          (CallFunction|RefreshJoinGame)
          (else
            (bind _array_element (Utilities|Array|ForEachLoopwithBreak _results :!label _label)
              (:LoopBody
                (if (< (Class|FindSessionsCallbackProxy|GetCurrentPlayers _array_element) (Class|FindSessionsCallbackProxy|GetMaxPlayers _array_element))
                  (Development|PrintString (Utilities|String|ToString(Integer) (Class|FindSessionsCallbackProxy|GetMaxPlayers _array_element)))
                  (|DestroySession _returnvalue
                    (:OnSuccess
                      _)
                    (:OnFailure
                      _))
                  (|JoinSession _returnvalue _array_element
                    (:OnSuccess
                      (Development|PrintString "Game joined!")
                      (goto _label Break)))
                  (else
                    (Development|PrintString "NOT ENOUGH ROOM!!!!!!!!!!!!"))))
              (:Completed
                (CallFunction|RefreshJoinGame)))))))
    (:OnFailure
      (CallFunction|RefreshJoinGame))))

(event EventBeginPlay
  (Utilities|FlowControl|Sequence
    (:then_0
      (bind _returnvalue (UserInterface|CreateWidget "/Game/UI/UMG_MainMenu_New.UMG_MainMenu_New_C"))
      (bind _output_get (Variables|Default|SetMainMenuUI _returnvalue))
      (UserInterface|Viewport|AddtoViewport _output_get 0)
      (Class|WidgetBlueprintLibrary|SetFocustoGameViewport)
      (Input|EnableInput (Game|GetPlayerController 0)))
    (:then_1
      (if (Utilities|Enum|Equal(Enum) (.RightS (Utilities|String|Split (Variables|/Script/Engine.GameModeBase|GetOptionsString (Game|GetGameMode)) "?")) "listen")
        (CallFunction|SelectWarrior)
        (else
          (bind _returnvalue_2 (Class|MainMenuManager|HasJoinedServer))
          (if _returnvalue_2
            (CallFunction|SelectBothHeroes)
            (Variables|Default|SetGameStarting true)
            (else
              (|DestroySession (Game|GetPlayerController 0)
                (:then
                  (CallFunction|FocusWarrior))))))))))

(event Collision|EventActorBeginOverlap
  (params (OtherActor :type Actor%20Object%20Reference)))

(event EventOnPlayerJoined
  (params (playerController :type Player%20Controller%20Object%20Reference))
  (Development|PrintString "PLAYER JOINED!!!")
  (Networking|SwitchHasAuthority
    (:Authority
      (if (== (Utilities|Array|Length (Variables|/Script/Engine.GameStateBase|GetPlayerArray (Game|GetGameState))) 2)
        (Variables|Default|SetGameStarting true)
        (CallFunction|SelectBothHeroes)
        (Utilities|FlowControl|Delay 1.0)
        (Game|LoadStreamLevel(byName) "/Game/Levels/00101_CenturianMineTemple" false)
        (CallFunction|RemoveMainMenuUI)))))

(event Input|ActionEvents|InputActionUnselectMenuOption
  (params (Key :type Key%20Structure :default "AnyKey"))
  (:Pressed
    (if (not (Variables|Default|GetGameStarting))
      (if (Variables|Default|GetWarriorFocused)
        (CallFunction|UnselectWarrior)
        (|DestroySession (Game|GetPlayerController 0))
        (else
          (CallFunction|UnselectMage))))))

(event Input|ActionEvents|InputActionSelectMenuOption
  (params (Key :type Key%20Structure :default "AnyKey"))
  (:Pressed
    (if (and (not (Variables|Default|GetHeroSelected)) (not (Variables|Default|GetGameStarting)))
      (if (Variables|Default|GetWarriorFocused)
        (CallFunction|RefreshCreateGame)
        (CallFunction|SelectWarrior)
        (else
          (CallFunction|RefreshJoinGame)
          (CallFunction|SelectMage))))))

(event Input|AxisEvents|InputAxisFocusNextOption
  (params (AxisValue :type Float%20%28single-precision%29))
  (if (Math|Boolean|ANDBoolean (> AxisValue 0.9) (Variables|Default|GetWarriorFocused) (not (Variables|Default|GetHeroSelected)))
    (CallFunction|FocusMage)))

(event Input|AxisEvents|InputAxisFocusPrevOption
  (params (AxisValue :type Float%20%28single-precision%29))
  (if (Math|Boolean|ANDBoolean (> AxisValue 0.9) (not (Variables|Default|GetWarriorFocused)) (not (Variables|Default|GetHeroSelected)))
    (CallFunction|FocusWarrior)))

(fn ConstructionScript)

(fn OnRepMageReady)

(fn FocusWarrior
  (bind _mainmenuui (Variables|Default|GetMainMenuUI))
  (Widget|SetVisibility (Variables|/Game/UI/UMG_MainMenu_New.UMG_MainMenu_New_C|GetFocusedWarriorImage _mainmenuui) "Visible")
  (Widget|SetVisibility (Variables|/Game/UI/UMG_MainMenu_New.UMG_MainMenu_New_C|GetFocusedMageImage _mainmenuui) "Hidden")
  (Variables|Default|SetWarriorFocused true))

(fn FocusMage
  (bind _mainmenuui (Variables|Default|GetMainMenuUI))
  (Widget|SetVisibility (Variables|/Game/UI/UMG_MainMenu_New.UMG_MainMenu_New_C|GetFocusedMageImage _mainmenuui) "Visible")
  (Widget|SetVisibility (Variables|/Game/UI/UMG_MainMenu_New.UMG_MainMenu_New_C|GetFocusedWarriorImage _mainmenuui) "Hidden")
  (Variables|Default|SetWarriorFocused false))

(fn SelectMage
  (bind _mainmenuui (Variables|Default|GetMainMenuUI))
  (Widget|SetVisibility (Variables|/Game/UI/UMG_MainMenu_New.UMG_MainMenu_New_C|GetSelectedMageImage _mainmenuui) "Visible")
  (Widget|SetVisibility (Variables|/Game/UI/UMG_MainMenu_New.UMG_MainMenu_New_C|GetFocusedMageImage _mainmenuui) "Hidden")
  (Widget|SetVisibility (Variables|/Game/UI/UMG_MainMenu_New.UMG_MainMenu_New_C|GetWarriorLoadingGif _mainmenuui) "Visible")
  (Variables|Default|SetHeroSelected true))

(fn SelectWarrior
  (bind _mainmenuui (Variables|Default|GetMainMenuUI))
  (Widget|SetVisibility (Variables|/Game/UI/UMG_MainMenu_New.UMG_MainMenu_New_C|GetSelectedWarriorImage _mainmenuui) "Visible")
  (Widget|SetVisibility (Variables|/Game/UI/UMG_MainMenu_New.UMG_MainMenu_New_C|GetFocusedWarriorImage _mainmenuui) "Hidden")
  (Widget|SetVisibility (Variables|/Game/UI/UMG_MainMenu_New.UMG_MainMenu_New_C|GetMageLoadingGif _mainmenuui) "Visible")
  (Variables|Default|SetHeroSelected true))

(fn UnselectMage
  (bind _mainmenuui (Variables|Default|GetMainMenuUI))
  (if (Math|Boolean|ANDBoolean (Variables|Default|GetHeroSelected) (not (Variables|Default|GetWarriorFocused)) (not (Variables|Default|GetGameStarting)))
    (Widget|SetVisibility (Variables|/Game/UI/UMG_MainMenu_New.UMG_MainMenu_New_C|GetSelectedMageImage _mainmenuui) "Hidden")
    (Widget|SetVisibility (Variables|/Game/UI/UMG_MainMenu_New.UMG_MainMenu_New_C|GetFocusedMageImage _mainmenuui) "Visible")
    (Widget|SetVisibility (Variables|/Game/UI/UMG_MainMenu_New.UMG_MainMenu_New_C|GetWarriorLoadingGif _mainmenuui) "Hidden")
    (Variables|Default|SetHeroSelected false)))

(fn UnselectWarrior
  (bind _mainmenuui (Variables|Default|GetMainMenuUI))
  (if (Math|Boolean|ANDBoolean (Variables|Default|GetHeroSelected) (Variables|Default|GetWarriorFocused) (not (Variables|Default|GetGameStarting)))
    (Widget|SetVisibility (Variables|/Game/UI/UMG_MainMenu_New.UMG_MainMenu_New_C|GetSelectedWarriorImage _mainmenuui) "Hidden")
    (Widget|SetVisibility (Variables|/Game/UI/UMG_MainMenu_New.UMG_MainMenu_New_C|GetFocusedWarriorImage _mainmenuui) "Visible")
    (Widget|SetVisibility (Variables|/Game/UI/UMG_MainMenu_New.UMG_MainMenu_New_C|GetMageLoadingGif _mainmenuui) "Hidden")
    (Variables|Default|SetHeroSelected false)))

(fn SelectBothHeroes
  (bind _mainmenuui (Variables|Default|GetMainMenuUI))
  (bind _mainmenuui_2 (Variables|Default|GetMainMenuUI))
  (Widget|SetVisibility (Variables|/Game/UI/UMG_MainMenu_New.UMG_MainMenu_New_C|GetSelectedMageImage _mainmenuui) "Visible")
  (Widget|SetVisibility (Variables|/Game/UI/UMG_MainMenu_New.UMG_MainMenu_New_C|GetFocusedMageImage _mainmenuui) "Hidden")
  (Widget|SetVisibility (Variables|/Game/UI/UMG_MainMenu_New.UMG_MainMenu_New_C|GetSelectedWarriorImage _mainmenuui_2) "Visible")
  (Widget|SetVisibility (Variables|/Game/UI/UMG_MainMenu_New.UMG_MainMenu_New_C|GetFocusedWarriorImage _mainmenuui_2) "Hidden")
  (Widget|SetVisibility (Variables|/Game/UI/UMG_MainMenu_New.UMG_MainMenu_New_C|GetMageLoadingGif _mainmenuui_2) "Hidden")
  (Widget|SetVisibility (Variables|/Game/UI/UMG_MainMenu_New.UMG_MainMenu_New_C|GetWarriorLoadingGif _mainmenuui_2) "Hidden")
  (Variables|Default|SetHeroSelected true))
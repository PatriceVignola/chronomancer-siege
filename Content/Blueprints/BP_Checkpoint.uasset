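; BP_Checkpoint is a one-time checkpoint that recharges the players when an actor first overlaps it.
; A DoOnce consumes the first overlap from any actor, then a Sequence calls RechargePlayers and posts the BurstAK Wwise event.
; The Circle effect activates for a short delay only if that actor is a Warrior or Mage character.
; Recharge and sound are not gated by those casts.
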(event EventBeginPlay)

(event Collision|EventActorBeginOverlap
  (params (OtherActor :type Actor%20Object%20Reference))
  (bind _circle (Variables|Default|GetCircle))
  (bind _circle_2 (Variables|Default|GetCircle))
  (Utilities|FlowControl|DoOnce false
    (:Completed
      (Utilities|FlowControl|Sequence
        (:then_0
          (Utilities|Casting|CastToBP_WarriorCharacter OtherActor)
          (Components|Activation|Activate _circle false)
          (Utilities|FlowControl|Delay 1.5)
          (Components|Activation|Deactivate _circle))
        (:then_1
          (Utilities|Casting|CastToBP_MageCharacter OtherActor)
          (Components|Activation|Activate _circle_2 false)
          (Utilities|FlowControl|Delay 1.5)
          (Components|Activation|Deactivate _circle_2))
        (:then_2
          (Class|Checkpoint|RechargePlayers))
        (:then_3
          (Class|AkComponent|PostAssociatedAkEvent (Variables|Default|GetBurstAK)))))))

(event EventTick
  (params (DeltaSeconds :type Float%20%28single-precision%29)))

(fn ConstructionScript)
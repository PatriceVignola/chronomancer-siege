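; Component that gives its owning pawn health and an on-screen health bar.
; On BeginPlay it creates a HealthBar2 widget in the viewport when the owner is a player-controlled pawn, then sets health to its maximum.
; A binding to the health-changed event updates the bar with the current health fraction.
; The file contains no damage logic, only initialization and display.
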(event Custom|OnHealthChangedEvent
  (params (health :type Float%20%28single-precision%29))
  (Default|SetPercent (Variables|Default|GetHealthBarWidget) (/ health (Variables|Default|GetMaxHealth))))

(event EventBeginPlay
  (CallFunction|AddLifeBar)
  (EventDispatchers|BindEventtoOnHealthChanged (delegate Custom|OnHealthChangedEvent))
  (bind _output_get (Variables|Default|SetMaxHealth 1e+02))
  (Class|DamageableCharacterComponent|SetHealth _output_get))

(fn AddLifeBar
  (bind _aspawn (Utilities|Casting|CastToPawn (Components|GetOwner)))
  (bind _asplayer_controller (Utilities|Casting|CastToPlayerController (Pawn|GetController _aspawn)))
  (bind _returnvalue (UserInterface|CreateWidget "/Game/UI/UI_elements/HealthBar2.HealthBar2_C" _asplayer_controller))
  (bind _output_get (Variables|Default|SetHealthBarWidget _returnvalue))
  (UserInterface|Viewport|AddtoViewport _output_get 0))
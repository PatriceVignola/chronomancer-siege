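; Energy component for a mage pawn that displays energy as mana crystals on the player's HUD.
; On BeginPlay, for player-controlled pawns, it creates the Mag_UI widget if BP_DamageableMage has none, stores it there, then binds the energy-changed delegate.
; EnergyChangedEvent converts the energy-to-max ratio into a whole crystal count and fills that shared widget.
; The EnergyChanged handler that BeginPlay binds and calls is empty here.
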(event Custom|EnergyChanged
  (params (NewEnergy :type Float%20%28single-precision%29)))

(event EventBeginPlay
  (bind _returnvalue (Components|GetOwner))
  (bind _returnvalue_2 (Actor|GetComponentbyClass _returnvalue "/Game/Blueprints/Components/BP_DamageableMage.BP_DamageableMage_C"))
  (bind _aspawn (Utilities|Casting|CastToPawn (Components|GetOwner)))
  (bind _asplayer_controller (Utilities|Casting|CastToPlayerController (Pawn|GetController _aspawn)))
  (if (Utilities|IsValid (Variables|/Game/Blueprints/Components/BP_DamageableMage.BP_DamageableMage_C|GetHealthBarWidget _returnvalue_2))
    _
    (else
      (bind _returnvalue_3 (UserInterface|CreateWidget "/Game/UI/Mag_UI.Mag_UI_C" _asplayer_controller))
      (bind _output_get (Variables|/Game/Blueprints/Components/BP_DamageableMage.BP_DamageableMage_C|SetHealthBarWidget _returnvalue_2 _returnvalue_3))
      (UserInterface|Viewport|AddtoViewport _output_get 0)))
  (EventDispatchers|BindEventtoOnEnergyChangedEvent (delegate Custom|EnergyChanged))
  (CallFunction|EnergyChanged (Variables|Default|GetInitialEnergy)))

(event EventTick
  (params (DeltaSeconds :type Float%20%28single-precision%29)))

(event EventEnergyChangedEvent
  (params (EnergyAmount :type Float%20%28single-precision%29))
  (bind _returnvalue (Components|GetOwner))
  (bind _returnvalue_2 (Actor|GetComponentbyClass _returnvalue "/Game/Blueprints/Components/BP_DamageableMage.BP_DamageableMage_C"))
  (bind _healthbarwidget (Variables|/Game/Blueprints/Components/BP_DamageableMage.BP_DamageableMage_C|GetHealthBarWidget _returnvalue_2))
  (Utilities|IsValid _healthbarwidget
    (:Is%20Valid
      (Default|FillEnergyCrystal _healthbarwidget (Math|Float|Truncate (/ (/ EnergyAmount (Variables|Default|GetMaxEnergy)) (/ 1.0 (Math|Conversions|ToFloat(Integer) (Variables|/Game/UI/Mag_UI.Mag_UI_C|GetnbOfManaCrystals _healthbarwidget)))))))))
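; Damageable component for the Warrior that creates a health HUD showing both Warrior and Mage health.
; On BeginPlay it adds the Warrior_UI widget for the owning player controller, or waits for the game mode's level-streaming event and adds it through an RPC.
; Setup resets health to max and binds both characters' health-change events, which push normalized values to the widget.
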(event Custom|RPC_AddLifeUI
  (bind _healthbarwidget (Variables|Default|GetHealthBarWidget))
  (CallFunction|AddLifeUI)
  (EventDispatchers|AssignOnWarriorHealthChange (delegate Custom|OnWarriorHealth))
  (EventDispatchers|AssignOnMageHealthChange (delegate Custom|OnMageHealth))
  (Class|DamageableCharacterComponent|SetHealth (Variables|Default|GetMaxHealth))
  (Utilities|IsValid _healthbarwidget
    (:Is%20Valid
      (Default|SetMageHealth _healthbarwidget 1.0)
      (Default|SetWarriorHealth (Variables|Default|GetHealthBarWidget) 1.0))))

(event Custom|OnLevelFinishedStreaming_Event_0
  (CallFunction|RPCAddLifeUI))

(event Custom|OnMageHealth
  (params (currentHealth :type Float%20%28single-precision%29) (MaxHealth :type Float%20%28single-precision%29))
  (bind _healthbarwidget (Variables|Default|GetHealthBarWidget))
  (Utilities|IsValid _healthbarwidget
    (:Is%20Valid
      (Default|SetMageHealth _healthbarwidget (/ currentHealth MaxHealth)))))

(event Custom|OnWarriorHealth
  (params (currentHealth :type Float%20%28single-precision%29) (MaxHealth :type Float%20%28single-precision%29))
  (bind _healthbarwidget (Variables|Default|GetHealthBarWidget))
  (Utilities|IsValid _healthbarwidget
    (:Is%20Valid
      (Default|SetWarriorHealth _healthbarwidget (/ currentHealth MaxHealth)))))

(event EventBeginPlay
  (bind _healthbarwidget (Variables|Default|GetHealthBarWidget))
  (bind _asbp_academia_2017game_mode (Utilities|Casting|CastToBP_Academia2017GameMode (Game|GetGameMode))
    (:then
      (if (Variables|/Script/Academia2017.Academia2017GameMode|GetHasBeenLevelStreamed _asbp_academia_2017game_mode)
        (EventDispatchers|AssignOnLevelFinishedStreaming _asbp_academia_2017game_mode (delegate Custom|OnLevelFinishedStreaming_Event_0))
        (else
          (CallFunction|AddLifeUI :!label _label))))
    (:CastFailed
      (goto _label)))
  (EventDispatchers|AssignOnWarriorHealthChange (delegate Custom|OnWarriorHealth))
  (EventDispatchers|AssignOnMageHealthChange (delegate Custom|OnMageHealth))
  (Class|DamageableCharacterComponent|SetHealth (Variables|Default|GetMaxHealth))
  (Utilities|IsValid _healthbarwidget
    (:Is%20Valid
      (Default|SetMageHealth _healthbarwidget 1.0)
      (Default|SetWarriorHealth (Variables|Default|GetHealthBarWidget) 1.0))))

(event EventTick
  (params (DeltaSeconds :type Float%20%28single-precision%29)))

(fn AddLifeUI
  (bind _aspawn (Utilities|Casting|CastToPawn (Components|GetOwner)))
  (bind _asplayer_controller (Utilities|Casting|CastToPlayerController (Pawn|GetController _aspawn)))
  (bind _returnvalue (UserInterface|CreateWidget "/Game/UI/Warrior_UI.Warrior_UI_C" _asplayer_controller))
  (bind _output_get (Variables|Default|SetHealthBarWidget _returnvalue))
  (UserInterface|Viewport|AddtoViewport _output_get 0))
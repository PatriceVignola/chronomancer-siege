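; Component that spawns and fades the mage or warrior pause menu, chosen by the owning character class.
; Focus and select events highlight Resume or Quit by toggling widget image visibility on whichever menu exists.
; Returning to the main menu goes through an RPC that disables input, fades in a class-specific loading screen, then reopens the PersistantRestart level as a listen server.
; Session-destroy and level-streaming exit paths remain but are never run.
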(event Custom|Server_RequestBackToMainMenu
  (CallFunction|RPCBacktoMainMenu))

(event Custom|RPC_BackToMainMenu
  (bind _returnvalue (Game|GetPlayerController 0))
  (Input|DisableInput _returnvalue _returnvalue)
  (Variables|Default|SetBackingToMainMenu true)
  (if (Utilities|IsValid (Variables|Default|GetPauseWarriorUI))
    (bind _returnvalue_2 (UserInterface|CreateWidget "/Game/UI/UMG_WarriorLoadingScreenNoControls.UMG_WarriorLoadingScreenNoControls_C" (Game|GetPlayerController 0) :!label _label))
    (bind _output_get (Variables|Default|SetWarriorLoadingScreen _returnvalue_2))
    (UserInterface|Viewport|AddtoViewport _output_get 10)
    (Utilities|FlowControl|Delay 0.2)
    (Default|Fadein (Variables|Default|GetWarriorLoadingScreen) 1.5)
    (Utilities|FlowControl|Delay 3.5)
    (elif (Utilities|IsValid (Variables|Default|GetPauseMageUI))
      (bind _returnvalue_3 (UserInterface|CreateWidget "/Game/UI/UMG_MageLoadingScreenNoControls.UMG_MageLoadingScreenNoControls_C" (Game|GetPlayerController 0)))
      (bind _output_get_2 (Variables|Default|SetMageLoadingScreen _returnvalue_3))
      (UserInterface|Viewport|AddtoViewport _output_get_2 10)
      (Utilities|FlowControl|Delay 0.2)
      (Default|Fadein (Variables|Default|GetMageLoadingScreen) 1.5)
      (Utilities|FlowControl|Delay 3.5)
      (else
        (goto _label))))
  (Game|OpenLevel(byName) "PersistantRestart" true "listen"))

(event EventTick
  (params (DeltaSeconds :type Float%20%28single-precision%29)))

(event EventBeginPlay)

(event EventFocusNextOption
  (Utilities|IsValid (Variables|Default|GetPauseMageUI)
    (:Is%20Valid
      (CallFunction|FocusMageQuit))
    (:Is%20Not%20Valid
      (Utilities|IsValid (Variables|Default|GetPauseWarriorUI)
        (:Is%20Valid
          (CallFunction|FocusWarriorQuit))))))

(event EventFocusPrevOption
  (Utilities|IsValid (Variables|Default|GetPauseMageUI)
    (:Is%20Valid
      (CallFunction|FocusMageResume))
    (:Is%20Not%20Valid
      (Utilities|IsValid (Variables|Default|GetPauseWarriorUI)
        (:Is%20Valid
          (CallFunction|FocusWarriorResume))))))

(event EventSelectResumeAction
  (Utilities|IsValid (Variables|Default|GetPauseMageUI)
    (:Is%20Valid
      (CallFunction|SelectMageResume))
    (:Is%20Not%20Valid
      (Utilities|IsValid (Variables|Default|GetPauseWarriorUI)
        (:Is%20Valid
          (CallFunction|SelectWarriorResume))))))

(event EventSelectQuitAction
  (Utilities|IsValid (Variables|Default|GetPauseMageUI)
    (:Is%20Valid
      (CallFunction|SelectMageQuit))
    (:Is%20Not%20Valid
      (Utilities|IsValid (Variables|Default|GetPauseWarriorUI)
        (:Is%20Valid
          (CallFunction|SelectWarriorQuit))))))

(event EventDespawn
  (params (playerController :type Player%20Controller%20Object%20Reference))
  (bind _pausewarriorui (Variables|Default|GetPauseWarriorUI))
  (bind _pausemageui (Variables|Default|GetPauseMageUI))
  (Utilities|IsValid _pausemageui
    (:Is%20Valid
      (Default|FadeOut _pausemageui 0.5 true))
    (:Is%20Not%20Valid
      (Utilities|IsValid _pausewarriorui
        (:Is%20Valid
          (Default|FadeOut _pausewarriorui 0.5 true))))))

(event EventSpawnPauseMenu
  (params (playerController :type Player%20Controller%20Object%20Reference))
  (bind _returnvalue (Components|GetOwner))
  (Utilities|IsValid playerController
    (:Is%20Valid
      (Utilities|Casting|CastToBP_MageCharacter _returnvalue
        (:then
          (Utilities|IsValid (Variables|Default|GetPauseMageUI)
            (:Is%20Valid
              _)
            (:Is%20Not%20Valid
              (bind _returnvalue_2 (UserInterface|CreateWidget "/Game/UI/UMG_PauseMage.UMG_PauseMage_C" playerController))
              (Variables|Default|SetPauseMageUI _returnvalue_2)))
          (Default|Fadein (Variables|Default|GetPauseMageUI) 0.5)
          (UserInterface|Viewport|AddtoViewport (Variables|Default|GetPauseMageUI) 0)
          (CallFunction|FocusMageResume))
        (:CastFailed
          (Utilities|Casting|CastToBP_WarriorCharacter _returnvalue)
          (Utilities|IsValid (Variables|Default|GetPauseWarriorUI)
            (:Is%20Valid
              _)
            (:Is%20Not%20Valid
              (bind _returnvalue_3 (UserInterface|CreateWidget "/Game/UI/UMG_PauseWarrior.UMG_PauseWarrior_C" playerController))
              (Variables|Default|SetPauseWarriorUI _returnvalue_3)))
          (Default|Fadein (Variables|Default|GetPauseWarriorUI) 0.5)
          (UserInterface|Viewport|AddtoViewport (Variables|Default|GetPauseWarriorUI) 0)
          (CallFunction|FocusWarriorResume))))))

(event EventBacktoMainMenu
  (if (not (Variables|Default|GetBackingToMainMenu))
    (Variables|Default|SetBackingToMainMenu true)
    (CallFunction|RPCBacktoMainMenu)))

(fn FocusWarriorResume
  (bind _pausewarriorui (Variables|Default|GetPauseWarriorUI))
  (Widget|SetVisibility (Variables|/Game/UI/UMG_PauseWarrior.UMG_PauseWarrior_C|GetSelectedQuit _pausewarriorui) "Hidden")
  (Widget|SetVisibility (Variables|/Game/UI/UMG_PauseWarrior.UMG_PauseWarrior_C|GetFocusQuit _pausewarriorui) "Hidden")
  (Widget|SetVisibility (Variables|/Game/UI/UMG_PauseWarrior.UMG_PauseWarrior_C|GetFocusResume _pausewarriorui) "Visible")
  (Widget|SetVisibility (Variables|/Game/UI/UMG_PauseWarrior.UMG_PauseWarrior_C|GetSelectedResume _pausewarriorui) "Hidden")
  (Widget|SetVisibility (Variables|/Game/UI/UMG_PauseWarrior.UMG_PauseWarrior_C|GetUnselectedQuit _pausewarriorui) "Visible")
  (Widget|SetVisibility (Variables|/Game/UI/UMG_PauseWarrior.UMG_PauseWarrior_C|GetUnselectedResume _pausewarriorui) "Hidden"))

(fn FocusWarriorQuit
  (bind _pausewarriorui (Variables|Default|GetPauseWarriorUI))
  (Widget|SetVisibility (Variables|/Game/UI/UMG_PauseWarrior.UMG_PauseWarrior_C|GetSelectedQuit _pausewarriorui) "Hidden")
  (Widget|SetVisibility (Variables|/Game/UI/UMG_PauseWarrior.UMG_PauseWarrior_C|GetFocusQuit _pausewarriorui) "Visible")
  (Widget|SetVisibility (Variables|/Game/UI/UMG_PauseWarrior.UMG_PauseWarrior_C|GetFocusResume _pausewarriorui) "Hidden")
  (Widget|SetVisibility (Variables|/Game/UI/UMG_PauseWarrior.UMG_PauseWarrior_C|GetSelectedResume _pausewarriorui) "Hidden")
  (Widget|SetVisibility (Variables|/Game/UI/UMG_PauseWarrior.UMG_PauseWarrior_C|GetUnselectedQuit _pausewarriorui) "Hidden")
  (Widget|SetVisibility (Variables|/Game/UI/UMG_PauseWarrior.UMG_PauseWarrior_C|GetUnselectedResume _pausewarriorui) "Visible"))

(fn SelectWarriorResume
  (bind _pausewarriorui (Variables|Default|GetPauseWarriorUI))
  (Widget|SetVisibility (Variables|/Game/UI/UMG_PauseWarrior.UMG_PauseWarrior_C|GetSelectedQuit _pausewarriorui) "Hidden")
  (Widget|SetVisibility (Variables|/Game/UI/UMG_PauseWarrior.UMG_PauseWarrior_C|GetFocusQuit _pausewarriorui) "Hidden")
  (Widget|SetVisibility (Variables|/Game/UI/UMG_PauseWarrior.UMG_PauseWarrior_C|GetFocusResume _pausewarriorui) "Hidden")
  (Widget|SetVisibility (Variables|/Game/UI/UMG_PauseWarrior.UMG_PauseWarrior_C|GetSelectedResume _pausewarriorui) "Visible")
  (Widget|SetVisibility (Variables|/Game/UI/UMG_PauseWarrior.UMG_PauseWarrior_C|GetUnselectedQuit _pausewarriorui) "Visible")
  (Widget|SetVisibility (Variables|/Game/UI/UMG_PauseWarrior.UMG_PauseWarrior_C|GetUnselectedResume _pausewarriorui) "Hidden"))

(fn SelectWarriorQuit
  (bind _pausewarriorui (Variables|Default|GetPauseWarriorUI))
  (Widget|SetVisibility (Variables|/Game/UI/UMG_PauseWarrior.UMG_PauseWarrior_C|GetSelectedQuit _pausewarriorui) "Visible")
  (Widget|SetVisibility (Variables|/Game/UI/UMG_PauseWarrior.UMG_PauseWarrior_C|GetFocusQuit _pausewarriorui) "Hidden")
  (Widget|SetVisibility (Variables|/Game/UI/UMG_PauseWarrior.UMG_PauseWarrior_C|GetFocusResume _pausewarriorui) "Hidden")
  (Widget|SetVisibility (Variables|/Game/UI/UMG_PauseWarrior.UMG_PauseWarrior_C|GetSelectedResume _pausewarriorui) "Hidden")
  (Widget|SetVisibility (Variables|/Game/UI/UMG_PauseWarrior.UMG_PauseWarrior_C|GetUnselectedQuit _pausewarriorui) "Hidden")
  (Widget|SetVisibility (Variables|/Game/UI/UMG_PauseWarrior.UMG_PauseWarrior_C|GetUnselectedResume _pausewarriorui) "Visible"))

(fn FocusMageResume
  (bind _pausemageui (Variables|Default|GetPauseMageUI))
  (Widget|SetVisibility (Variables|/Game/UI/UMG_PauseMage.UMG_PauseMage_C|GetSelectedQuit _pausemageui) "Hidden")
  (Widget|SetVisibility (Variables|/Game/UI/UMG_PauseMage.UMG_PauseMage_C|GetFocusQuit _pausemageui) "Hidden")
  (Widget|SetVisibility (Variables|/Game/UI/UMG_PauseMage.UMG_PauseMage_C|GetFocusResume _pausemageui) "Visible")
  (Widget|SetVisibility (Variables|/Game/UI/UMG_PauseMage.UMG_PauseMage_C|GetSelectedResume _pausemageui) "Hidden")
  (Widget|SetVisibility (Variables|/Game/UI/UMG_PauseMage.UMG_PauseMage_C|GetUnselectedQuit _pausemageui) "Visible")
  (Widget|SetVisibility (Variables|/Game/UI/UMG_PauseMage.UMG_PauseMage_C|GetUnselectedResume _pausemageui) "Hidden"))

(fn FocusMageQuit
  (bind _pausemageui (Variables|Default|GetPauseMageUI))
  (Widget|SetVisibility (Variables|/Game/UI/UMG_PauseMage.UMG_PauseMage_C|GetSelectedQuit _pausemageui) "Hidden")
  (Widget|SetVisibility (Variables|/Game/UI/UMG_PauseMage.UMG_PauseMage_C|GetFocusQuit _pausemageui) "Visible")
  (Widget|SetVisibility (Variables|/Game/UI/UMG_PauseMage.UMG_PauseMage_C|GetFocusResume _pausemageui) "Hidden")
  (Widget|SetVisibility (Variables|/Game/UI/UMG_PauseMage.UMG_PauseMage_C|GetSelectedResume _pausemageui) "Hidden")
  (Widget|SetVisibility (Variables|/Game/UI/UMG_PauseMage.UMG_PauseMage_C|GetUnselectedQuit _pausemageui) "Hidden")
  (Widget|SetVisibility (Variables|/Game/UI/UMG_PauseMage.UMG_PauseMage_C|GetUnselectedResume _pausemageui) "Visible"))

(fn SelectMageResume
  (bind _pausemageui (Variables|Default|GetPauseMageUI))
  (Widget|SetVisibility (Variables|/Game/UI/UMG_PauseMage.UMG_PauseMage_C|GetSelectedQuit _pausemageui) "Hidden")
  (Widget|SetVisibility (Variables|/Game/UI/UMG_PauseMage.UMG_PauseMage_C|GetFocusQuit _pausemageui) "Hidden")
  (Widget|SetVisibility (Variables|/Game/UI/UMG_PauseMage.UMG_PauseMage_C|GetFocusResume _pausemageui) "Hidden")
  (Widget|SetVisibility (Variables|/Game/UI/UMG_PauseMage.UMG_PauseMage_C|GetSelectedResume _pausemageui) "Visible")
  (Widget|SetVisibility (Variables|/Game/UI/UMG_PauseMage.UMG_PauseMage_C|GetUnselectedQuit _pausemageui) "Visible")
  (Widget|SetVisibility (Variables|/Game/UI/UMG_PauseMage.UMG_PauseMage_C|GetUnselectedResume _pausemageui) "Hidden"))

(fn SelectMageQuit
  (bind _pausemageui (Variables|Default|GetPauseMageUI))
  (Widget|SetVisibility (Variables|/Game/UI/UMG_PauseMage.UMG_PauseMage_C|GetSelectedQuit _pausemageui) "Visible")
  (Widget|SetVisibility (Variables|/Game/UI/UMG_PauseMage.UMG_PauseMage_C|GetFocusQuit _pausemageui) "Hidden")
  (Widget|SetVisibility (Variables|/Game/UI/UMG_PauseMage.UMG_PauseMage_C|GetFocusResume _pausemageui) "Hidden")
  (Widget|SetVisibility (Variables|/Game/UI/UMG_PauseMage.UMG_PauseMage_C|GetSelectedResume _pausemageui) "Hidden")
  (Widget|SetVisibility (Variables|/Game/UI/UMG_PauseMage.UMG_PauseMage_C|GetUnselectedQuit _pausemageui) "Hidden")
  (Widget|SetVisibility (Variables|/Game/UI/UMG_PauseMage.UMG_PauseMage_C|GetUnselectedResume _pausemageui) "Visible"))
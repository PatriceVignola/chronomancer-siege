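; Component that shows on-screen tutorial prompt widgets for characters and abilities such as Kalika, Aion, combo, clone time, slow time and healing.
; The spawn event switches on the tutorial type, creating, storing and fading in the matching widget, with a DoOnce limiting each to one appearance.
; It also posts a Wwise spawn sound at the owner's location.
; The despawn event fades out every valid stored widget without removing it itself.
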(event EventBPDespawn
  (bind _kalikawidget (Variables|Default|GetKalikaWidget))
  (bind _combowidget (Variables|Default|GetComboWidget))
  (bind _clonetimewarriorwidget (Variables|Default|GetCloneTimeWarriorWidget))
  (bind _aionwidget (Variables|Default|GetAionWidget))
  (bind _clonetimewidget (Variables|Default|GetCloneTimeWidget))
  (bind _slowwidget (Variables|Default|GetSlowWidget))
  (bind _healingwidget (Variables|Default|GetHealingWidget))
  ;[1 1 1] Despawn
  (Utilities|IsValid _kalikawidget
    (:Is%20Valid
      (Default|FadeOut _kalikawidget 0.5))
    (:Is%20Not%20Valid
      _))
  (Utilities|IsValid _combowidget
    (:Is%20Valid
      (Default|FadeOut _combowidget 0.5))
    (:Is%20Not%20Valid
      _))
  (Utilities|IsValid _clonetimewarriorwidget
    (:Is%20Valid
      (Default|FadeOut _clonetimewarriorwidget 0.5))
    (:Is%20Not%20Valid
      _))
  (Utilities|IsValid _aionwidget
    (:Is%20Valid
      (Default|FadeOut _aionwidget 0.5))
    (:Is%20Not%20Valid
      _))
  (Utilities|IsValid _clonetimewidget
    (:Is%20Valid
      (Default|FadeOut _clonetimewidget 0.5))
    (:Is%20Not%20Valid
      _))
  (Utilities|IsValid _slowwidget
    (:Is%20Valid
      (Default|FadeOut _slowwidget 0.5))
    (:Is%20Not%20Valid
      _))
  (Utilities|IsValid _healingwidget
    (:Is%20Valid
      (Default|FadeOut _healingwidget 0.5))))

(event EventBPSpawnNextPrompt
  (params (Tutorial :type TutorialPrompt%20Enum :default "Kalika") (playerController :type Player%20Controller%20Object%20Reference))
  ;[1 1 1] Spawn
  (Utilities|IsValid playerController
    (:Is%20Valid
      (switch Utilities|FlowControl|Switch|SwitchonTutorialPrompt Tutorial
        (:Kalika
          (Utilities|FlowControl|DoOnce false
            (:Completed
              (bind _returnvalue (UserInterface|CreateWidget "/Game/UI/UI_elements/flipbook/flipbookController/Prompts_Kalika.Prompts_Kalika_C" playerController))
              (bind _output_get (Variables|Default|SetKalikaWidget _returnvalue))
              (Default|Fadein _output_get 0.5)
              (UserInterface|Viewport|AddtoViewport _output_get 0))))
        (:Combo
          (Utilities|FlowControl|DoOnce false
            (:Completed
              (bind _returnvalue_2 (UserInterface|CreateWidget "/Game/UI/UI_elements/flipbook/flipbookController/Prompts_comboFight.Prompts_comboFight_C" playerController))
              (bind _output_get_2 (Variables|Default|SetComboWidget _returnvalue_2))
              (Default|Fadein _output_get_2 0.5)
              (UserInterface|Viewport|AddtoViewport _output_get_2 0))))
        (:KalikaCloneTime
          (Utilities|FlowControl|DoOnce false
            (:Completed
              (bind _returnvalue_3 (UserInterface|CreateWidget "/Game/UI/UI_elements/flipbook/flipbookController/Prompts_CloneTime_Warrior.Prompts_CloneTime_Warrior_C" playerController))
              (bind _output_get_3 (Variables|Default|SetCloneTimeWarriorWidget _returnvalue_3))
              (Default|Fadein _output_get_3 0.5)
              (UserInterface|Viewport|AddtoViewport _output_get_3 0))))
        (:Aion
          (Utilities|FlowControl|DoOnce false
            (:Completed
              (bind _returnvalue_4 (UserInterface|CreateWidget "/Game/UI/UI_elements/flipbook/flipbookController/Prompts_Aion.Prompts_Aion_C" playerController))
              (bind _output_get_4 (Variables|Default|SetAionWidget _returnvalue_4))
              (Default|Fadein _output_get_4 0.5)
              (UserInterface|Viewport|AddtoViewport _output_get_4 0))))
        (:CloneTime
          (Utilities|FlowControl|DoOnce false
            (:Completed
              (bind _returnvalue_5 (UserInterface|CreateWidget "/Game/UI/UI_elements/flipbook/flipbookController/Prompts_CloneTime.Prompts_CloneTime_C" playerController))
              (bind _output_get_5 (Variables|Default|SetCloneTimeWidget _returnvalue_5))
              (Default|Fadein _output_get_5 0.5)
              (UserInterface|Viewport|AddtoViewport _output_get_5 0))))
        (:SlowTime
          (Utilities|FlowControl|DoOnce false
            (:Completed
              (bind _returnvalue_6 (UserInterface|CreateWidget "/Game/UI/UI_elements/flipbook/flipbookController/Prompts_slow.Prompts_slow_C" playerController))
              (bind _output_get_6 (Variables|Default|SetSlowWidget _returnvalue_6))
              (Default|Fadein _output_get_6 0.5)
              (UserInterface|Viewport|AddtoViewport _output_get_6 0))))
        (:Heal
          (Utilities|FlowControl|DoOnce false
            (:Completed
              (bind _returnvalue_7 (UserInterface|CreateWidget "/Game/UI/UI_elements/flipbook/flipbookController/Prompts_Healing.Prompts_Healing_C" playerController))
              (bind _output_get_7 (Variables|Default|SetHealingWidget _returnvalue_7))
              (Default|Fadein _output_get_7 0.5)
              (UserInterface|Viewport|AddtoViewport _output_get_7 0)))))
      (Class|AkGameplayStatics|PostEventatLocation (Variables|Default|GetSpawnSound) (Transformation|GetActorLocation (Components|GetOwner)) "0, 0, 0"))))
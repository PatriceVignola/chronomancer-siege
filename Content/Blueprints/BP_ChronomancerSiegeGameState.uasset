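; Game state Blueprint for Chronomancer Siege that runs a black-screen overlay, fading it away to reveal the game.
; On authority, it binds to Academia2017GameMode events that create the overlay and start the timed fade.
; Tick counts down only on authority but sets overlay opacity from the remaining-time ratio on any machine where FadingOut is set.
; At zero, authority triggers the overlay-removal RPC and has the game mode enable inputs.
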(event Custom|OnBlackOverlayRequested_Event_0
  (CallFunction|CreateBlackOverlay))

(event Custom|OnStartFadingOut_Event_0
  (Networking|SwitchHasAuthority
    (:Authority
      (CallFunction|RPCStartFadingOut)
      (bind _asacademia_2017game_mode (Utilities|Casting|CastToAcademia2017GameMode (Game|GetGameMode)))
      (bind _output_get (Variables|Default|SetFadeOutRemainingDuration (Variables|/Script/Academia2017.Academia2017GameMode|GetFadeOutDuration _asacademia_2017game_mode)))
      (Variables|Default|SetFadeOutDuration _output_get)
      (Variables|Default|SetFadingOut true))))

(event Custom|CreateBlackOverlay
  (bind _returnvalue (UserInterface|CreateWidget "/Game/UI/UMG_BlackOverlay.UMG_BlackOverlay_C" (Game|GetPlayerController 0)))
  (bind _output_get (Variables|Default|SetBlackOverlay _returnvalue))
  (UserInterface|Viewport|AddtoViewport _output_get 0))

(event Custom|RPC_StopFadingOut
  (Widget|RemovefromParent (Variables|Default|GetBlackOverlay)))

(event Custom|RPC_StartFadingOut
  (Development|PrintString "Start Fading Out In Blueprint"))

(event EventBeginPlay
  (Networking|SwitchHasAuthority
    (:Authority
      (bind _asacademia_2017game_mode (Utilities|Casting|CastToAcademia2017GameMode (Game|GetGameMode)))
      (EventDispatchers|AssignOnStartFadingOut _asacademia_2017game_mode (delegate Custom|OnStartFadingOut_Event_0))
      (EventDispatchers|AssignOnBlackOverlayRequested _asacademia_2017game_mode (delegate Custom|OnBlackOverlayRequested_Event_0)))))

(event EventTick
  (params (DeltaSeconds :type Float%20%28single-precision%29))
  (if (Variables|Default|GetFadingOut)
    (Networking|SwitchHasAuthority
      (:Authority
        (bind _output_get (Variables|Default|SetFadeOutRemainingDuration (- (Variables|Default|GetFadeOutRemainingDuration) DeltaSeconds))))
      (:Remote
        _))
    (Class|Image|SetOpacity (Variables|/Game/UI/UMG_BlackOverlay.UMG_BlackOverlay_C|GetBlackImage (Variables|Default|GetBlackOverlay)) (/ (Variables|Default|GetFadeOutRemainingDuration) (Variables|Default|GetFadeOutDuration)))
    (Networking|SwitchHasAuthority
      (:Authority
        (if (<= _output_get 0.0)
          (Variables|Default|SetFadingOut false)
          (CallFunction|RPCStopFadingOut)
          (bind _asacademia_2017game_mode (Utilities|Casting|CastToAcademia2017GameMode (Game|GetGameMode)))
          (Class|Academia2017GameMode|EnableInputs _asacademia_2017game_mode))))))

(fn ConstructionScript)